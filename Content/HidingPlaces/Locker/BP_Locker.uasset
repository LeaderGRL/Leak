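; BP_Locker is an interactable hiding locker that highlights on focus and hides or releases the first-person character.
; An interact call toggles a RepNotify variable that runs the hide logic through a gate controlled by box overlap.
; Hiding disables the character's movement, visibility and collision, then blends view to the locker.
; While hidden, look input sets clamped yaw and pitch, applied by a self-calling delay loop, and interact input exits.
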(event OnComponentBeginOverlap(Box)
  (params (OverlappedComponent :type Primitive%20Component%20Object%20Reference) (OtherActor :type Actor%20Object%20Reference) (OtherComp :type Primitive%20Component%20Object%20Reference) (OtherBodyIndex :type Integer) (bFromSweep :type Boolean) (SweepResult :type Hit%20Result%20Structure%20%28by%20ref%29))
  ;[0 1 0.4375] Enable Hiding
  (bind _asbp_first_person_character (Utilities|Casting|CastToBP_FirstPersonCharacter OtherActor))
  (Variables|Hiding|SetCharREF _asbp_first_person_character)
  (Variables|Hiding|SetIsColliding? true)
  (Input|EnableInput (Game|GetPlayerController 0))
  ;[0.1016 1 0] if Hiding is enabled start or stop hiding
  (Utilities|FlowControl|Gate true) ; enters at Open
)

(event OnComponentEndOverlap(Box)
  (params (OverlappedComponent :type Primitive%20Component%20Object%20Reference) (OtherActor :type Actor%20Object%20Reference) (OtherComp :type Primitive%20Component%20Object%20Reference) (OtherBodyIndex :type Integer))
  (bind _returnvalue (Game|GetPlayerController 0))
  ;[0 1 0.4375] Disable Hiding
  (Utilities|Casting|CastToBP_FirstPersonCharacter OtherActor)
  (Variables|Hiding|SetIsColliding? false)
  (Input|DisableInput _returnvalue)
  ;[0.1016 1 0] if Hiding is enabled start or stop hiding
  (Utilities|FlowControl|Gate true) ; enters at Close
)

(event Custom|Unhide
  (bind _charref (Variables|Hiding|GetCharREF))
  (bind _charref_2 (Variables|Hiding|GetCharREF))
  ;[0 1 0.8594] Hide/Unhide
  (Variables|/Game/FirstPerson/Blueprints/BP_FirstPersonCharacter.BP_FirstPersonCharacter_C|SetIsHiding? _charref false)
  (Pawn|Components|CharacterMovement|SetMovementMode (Variables|/Script/Engine.Character|GetCharacterMovement _charref) "MOVE_Walking" 0)
  (Game|Player|SetViewTargetwithBlend (Game|GetPlayerController 0) (Variables|Hiding|GetCharREF) 0.5 "VTBlend_Linear" 0.0 false)
  (Utilities|FlowControl|Delay 0.5)
  (Rendering|SetActorHiddenInGame _charref_2 false)
  (Collision|SetCollisionEnabled (Variables|/Script/Engine.Character|GetCapsuleComponent _charref_2) "QueryAndProbe"))

(event Custom|Hide
  (bind _charref (Variables|Hiding|GetCharREF))
  (bind _charref_2 (Variables|Hiding|GetCharREF))
  ;[0 1 0.8594] Hide/Unhide
  (Variables|/Game/FirstPerson/Blueprints/BP_FirstPersonCharacter.BP_FirstPersonCharacter_C|SetIsHiding? _charref true)
  (Pawn|Components|CharacterMovement|DisableMovement (Variables|/Script/Engine.Character|GetCharacterMovement _charref))
  (Rendering|SetActorHiddenInGame _charref_2 true)
  (Collision|SetCollisionEnabled (Variables|/Script/Engine.Character|GetCapsuleComponent _charref_2) "NoCollision"))

(event Custom|MoveCamera
  ;[1 0.2812 0] Camera Input : Moving and limiting the camera
  (if (Variables|/Game/FirstPerson/Blueprints/BP_FirstPersonCharacter.BP_FirstPersonCharacter_C|GetIsHiding? (Variables|Hiding|GetCharREF))
    (Transformation|SetRelativeRotation (Variables|Default|GetCamera) (Math|Rotator|MakeRotator 0.0 (stale Input|EnhancedActionEvents|EnhancedInputActionIA_Look _output_get_2) (stale Input|EnhancedActionEvents|EnhancedInputActionIA_Look _output_get)) false false)
    (Utilities|FlowControl|Delay 0.001)
    (CallFunction|MoveCamera)))

(event Custom|Interract
  ;[0 1 0.4375] Start Hiding
  (if (Variables|Hiding|GetIsColliding?)
    ;[0.1016 1 0] if Hiding is enabled start or stop hiding
    (Utilities|FlowControl|Gate true :!label _label
      (:Exit
        (if (Variables|/Game/FirstPerson/Blueprints/BP_FirstPersonCharacter.BP_FirstPersonCharacter_C|GetIsHiding? (Variables|Hiding|GetCharREF))
          (CallFunction|Unhide)
          (else
            (CallFunction|Hide)
            (Utilities|FlowControl|Sequence
              (:then_0
                (Game|Player|SetViewTargetwithBlend (Game|GetPlayerController 0) self 0.5 "VTBlend_Linear" 0.0 false)
                (CallFunction|MoveCamera))
              (:then_1
                (Utilities|FlowControl|Delay 0.2)
                ;[0 1 0.4375] Enable Hiding
                (Input|EnableInput (Game|GetPlayerController 0))
                (goto _label Open)))))))
    (else
      (Development|PrintString "You're too far"))))

(event Custom|InteractOnServer
  ;[0 1 0.2031] Enable Interaction
  (Variables|Default|SetInteractToggle (not (Variables|Default|GetInteractToggle))))

(event Input|EnhancedActionEvents|EnhancedInputActionIA_Interact
  (params (ActionValue :type Boolean) (ElapsedSeconds :type Float%20%28double-precision%29) (TriggeredSeconds :type Float%20%28double-precision%29) (InputAction :type Input%20Action%20Object%20Reference :default "/Game/FirstPerson/Input/Actions/IA_Interact.IA_Interact"))
  ;[0 1 0.4375] Stop Hiding
  (:Started
    (if (Variables|/Game/FirstPerson/Blueprints/BP_FirstPersonCharacter.BP_FirstPersonCharacter_C|GetIsHiding? (Variables|Hiding|GetCharREF))
      ;[0.1016 1 0] if Hiding is enabled start or stop hiding
      (Utilities|FlowControl|Gate true :!label _label
        (:Exit
          (if (Variables|/Game/FirstPerson/Blueprints/BP_FirstPersonCharacter.BP_FirstPersonCharacter_C|GetIsHiding? (Variables|Hiding|GetCharREF))
            (CallFunction|Unhide)
            (else
              (CallFunction|Hide)
              (Utilities|FlowControl|Sequence
                (:then_0
                  (Game|Player|SetViewTargetwithBlend (Game|GetPlayerController 0) self 0.5 "VTBlend_Linear" 0.0 false)
                  (CallFunction|MoveCamera))
                (:then_1
                  (Utilities|FlowControl|Delay 0.2)
                  ;[0 1 0.4375] Enable Hiding
                  (Input|EnableInput (Game|GetPlayerController 0))
                  (goto _label Open))))))))))

(event Input|EnhancedActionEvents|EnhancedInputActionIA_Look
  (params (ActionValue :type Vector%202D%20Structure) (ElapsedSeconds :type Float%20%28double-precision%29) (TriggeredSeconds :type Float%20%28double-precision%29) (InputAction :type Input%20Action%20Object%20Reference :default "/Game/FirstPerson/Input/Actions/IA_Look.IA_Look"))
  ;[1 0.2812 0] Camera Input : Moving and limiting the camera
  (if (Variables|/Game/FirstPerson/Blueprints/BP_FirstPersonCharacter.BP_FirstPersonCharacter_C|GetIsHiding? (Variables|Hiding|GetCharREF))
    (Utilities|FlowControl|Sequence
      (:then_0
        ;;[0 1 0.7656] Yaw (Z)
        (bind _output_get (Variables|Hiding|SetYaw (Math|Float|Clamp(Float) (+ (.x ActionValue) (Variables|Hiding|GetYaw)) 6e+01 1.2e+02))))
      (:then_1
        ;;[0 1 0.7656] Pitch (Y)
        (bind _output_get_2 (Variables|Hiding|SetPitch (Math|Float|Clamp(Float) (+ (* (.y ActionValue) -1.0) (Variables|Hiding|GetPitch)) -1e+01 1e+01)))))))

(event EventInterfaceToggleFocus
  (params (Focus :type Boolean))
  ;[0 1 0.2031] Enable Interaction
  (Rendering|SetRenderCustomDepth (Variables|Default|GetSM_Locker_Door) Focus))

(event EventInterfaceInteract
  ;[0 1 0.2031] Enable Interaction
  (CallFunction|InteractonServer))

(fn ConstructionScript)

(fn OnRepInteractToggle
  (CallFunction|Interract))