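; Base hiding-place actor where the player character can hide and look out through a camera with clamped yaw and pitch.
; Interact toggles hiding by switching character visibility, movement and collision, and blending the view between actor and character.
; While hidden, look input updates the angles and a self-calling Delay loop applies them to the camera.
; The construction script applies configurable mesh, camera, widget and box settings, and configures a child interaction-area actor.
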(event Custom|Unhide
  (bind _charref (Variables|Hiding|GetCharREF))
  (bind _charref_2 (Variables|Hiding|GetCharREF))
  ;[0 1 0.8594] Hide/Unhide
  (Variables|/Game/FirstPerson/Blueprints/BP_FirstPersonCharacter.BP_FirstPersonCharacter_C|SetIsHiding? _charref false)
  (Pawn|Components|CharacterMovement|SetMovementMode (Variables|/Script/Engine.Character|GetCharacterMovement _charref) "MOVE_Walking" 0)
  (Game|Player|SetViewTargetwithBlend (Game|GetPlayerController 0) (Variables|Hiding|GetCharREF) 0.5 "VTBlend_Linear" 0.0 false)
  (Utilities|FlowControl|Delay 0.5)
  (Rendering|SetActorHiddenInGame _charref_2 false)
  (Collision|SetCollisionEnabled (Variables|/Script/Engine.Character|GetCapsuleComponent _charref_2) "QueryAndProbe"))

(event Custom|Hide
  (bind _charref (Variables|Hiding|GetCharREF))
  (bind _charref_2 (Variables|Hiding|GetCharREF))
  ;[0 1 0.8594] Hide/Unhide
  (Variables|/Game/FirstPerson/Blueprints/BP_FirstPersonCharacter.BP_FirstPersonCharacter_C|SetIsHiding? _charref true)
  (Pawn|Components|CharacterMovement|DisableMovement (Variables|/Script/Engine.Character|GetCharacterMovement _charref))
  (Rendering|SetActorHiddenInGame _charref_2 true)
  (Collision|SetCollisionEnabled (Variables|/Script/Engine.Character|GetCapsuleComponent _charref_2) "NoCollision"))

(event Custom|MoveCamera
  ;[1 0.2812 0] Camera Input : Moving and limiting the camera
  (if (Variables|/Game/FirstPerson/Blueprints/BP_FirstPersonCharacter.BP_FirstPersonCharacter_C|GetIsHiding? (Variables|Hiding|GetCharREF))
    (Transformation|SetRelativeRotation (Variables|Default|GetCamera) (Math|Rotator|MakeRotator 0.0 (stale Input|EnhancedActionEvents|EnhancedInputActionIA_Look _output_get_2) (stale Input|EnhancedActionEvents|EnhancedInputActionIA_Look _output_get)) false false)
    (Utilities|FlowControl|Delay 0.001)
    (CallFunction|MoveCamera)))

(event Custom|Interract
  (bind _returnvalue (Game|GetPlayerController 0))
  ;[0.1016 1 0] if Hiding is enabled start or stop hiding
  ;;[0.07812 1 0] Start Hiding
  (Input|EnableInput (Game|GetPlayerController 0))
  (if (Variables|/Game/FirstPerson/Blueprints/BP_FirstPersonCharacter.BP_FirstPersonCharacter_C|GetIsHiding? (Variables|Hiding|GetCharREF))
    (CallFunction|Unhide)
    (Input|DisableInput _returnvalue)
    (else
      (CallFunction|Hide)
      (Game|Player|SetViewTargetwithBlend _returnvalue self 0.5 "VTBlend_Linear" 0.0 false)
      (CallFunction|MoveCamera))))

(event Custom|InteractOnServer
  ;[0 1 0.2031] Enable Interaction
  (Variables|Default|SetInteractToggle (not (Variables|Default|GetInteractToggle))))

(event Input|EnhancedActionEvents|EnhancedInputActionIA_Interact
  (params (ActionValue :type Boolean) (ElapsedSeconds :type Float%20%28double-precision%29) (TriggeredSeconds :type Float%20%28double-precision%29) (InputAction :type Input%20Action%20Object%20Reference :default "/Game/FirstPerson/Input/Actions/IA_Interact.IA_Interact"))
  (bind _returnvalue (Game|GetPlayerController 0))
  ;[0.1016 1 0] if Hiding is enabled start or stop hiding
  ;;[0 1 0.4375] Stop Hiding
  (:Started
    (if (Variables|/Game/FirstPerson/Blueprints/BP_FirstPersonCharacter.BP_FirstPersonCharacter_C|GetIsHiding? (Variables|Hiding|GetCharREF))
      (if (Variables|/Game/FirstPerson/Blueprints/BP_FirstPersonCharacter.BP_FirstPersonCharacter_C|GetIsHiding? (Variables|Hiding|GetCharREF))
        (CallFunction|Unhide)
        (Input|DisableInput _returnvalue)
        (else
          (CallFunction|Hide)
          (Game|Player|SetViewTargetwithBlend _returnvalue self 0.5 "VTBlend_Linear" 0.0 false)
          (CallFunction|MoveCamera))))))

(event Input|EnhancedActionEvents|EnhancedInputActionIA_Look
  (params (ActionValue :type Vector%202D%20Structure) (ElapsedSeconds :type Float%20%28double-precision%29) (TriggeredSeconds :type Float%20%28double-precision%29) (InputAction :type Input%20Action%20Object%20Reference :default "/Game/FirstPerson/Input/Actions/IA_Look.IA_Look"))
  ;[1 0.2812 0] Camera Input : Moving and limiting the camera
  (if (Variables|/Game/FirstPerson/Blueprints/BP_FirstPersonCharacter.BP_FirstPersonCharacter_C|GetIsHiding? (Variables|Hiding|GetCharREF))
    (Utilities|FlowControl|Sequence
      (:then_0
        ;;[0 1 0.7656] Yaw (Z)
        (bind _output_get (Variables|Hiding|SetYaw (Math|Float|Clamp(Float) (+ (.x ActionValue) (Variables|Hiding|GetYaw)) (Variables|Init|GetMinYaw%20%28Z%29) (Variables|Init|GetMaxYaw%20%28Z%29)))))
      (:then_1
        ;;[0 1 0.7656] Pitch (Y)
        (bind _output_get_2 (Variables|Hiding|SetPitch (Math|Float|Clamp(Float) (+ (* (.y ActionValue) -1.0) (Variables|Hiding|GetPitch)) (Variables|Init|GetMinPitch%20%28Y%29) (Variables|Init|GetMaxPitch%20%28Y%29))))))))

(event EventInterfaceToggleFocus
  (params (Focus :type Boolean))
  ;[0 1 0.2031] Enable Interaction
  (Rendering|SetRenderCustomDepth (Variables|Default|GetStaticMesh) Focus))

(event EventInterfaceInteract
  ;[0 1 0.2031] Enable Interaction
  (CallFunction|InteractonServer))

(fn ConstructionScript
  (bind _camera (Variables|Default|GetCamera))
  (bind _camerarotation (Variables|Init|GetCameraRotation))
  (bind _box (Variables|Default|GetBox))
  (bind (_roll _pitch _yaw) (Math|Rotator|BreakRotator _camerarotation))
  (Utilities|FlowControl|Sequence
    (:then_0
      ;[0 1 0.9063] Set Static Mesh
      (Components|StaticMesh|SetStaticMesh (Variables|Default|GetStaticMesh) (Variables|Init|GetBasicMesh)))
    (:then_1
      ;[0 1 0.9062] Set Camera Parameters
      (Transformation|SetRelativeLocationAndRotation _camera (Variables|Init|GetCameraLocation) _camerarotation false false)
      (Variables|Hiding|SetPitch _pitch)
      (Variables|Hiding|SetYaw _yaw)
      (Camera|SetFieldOfView _camera (Variables|Init|GetCameraFOV)))
    (:then_2
      ;[0 1 0.9062] Set Widget Location
      (Transformation|SetRelativeLocation (Variables|Default|GetWidget) (Variables|Init|GetWidget%20Location) false false))
    (:then_3
      ;[0 1 0.9062] Set Box Collision Parameters
      (Transformation|SetRelativeScale3D _box (Variables|Init|GetBox%20Colision%20Scale))
      (Transformation|SetRelativeLocation _box (Variables|Init|GetBox%20Location) false false))
    (:then_4
      ;[0 1 0.9062] Set Child Actor Mesh
      (bind _asbp_interaction_area_custom_shape (Utilities|Casting|CastToBP_InteractionArea_Custom_Shape (Variables|/Script/Engine.ChildActorComponent|GetChildActor (Variables|Default|GetChildActor))))
      (Variables|/Game/Interaction/InteractionArea/BP_InteractionArea_Master.BP_InteractionArea_Master_C|SetInteractDuration _asbp_interaction_area_custom_shape (Variables|Init|GetInteract%20Duration))
      (Components|StaticMesh|SetStaticMesh (Variables|/Game/Interaction/InteractionArea/BP_InteractionArea_Custom_Shape.BP_InteractionArea_Custom_Shape_C|GetShape _asbp_interaction_area_custom_shape) (Variables|Init|GetBasicMesh))
      (Variables|/Game/Interaction/InteractionArea/BP_InteractionArea_Master.BP_InteractionArea_Master_C|SetCharNeedsToBeInBox _asbp_interaction_area_custom_shape (Variables|Init|GetChar%20Needs%20to%20be%20in%20Box)))))