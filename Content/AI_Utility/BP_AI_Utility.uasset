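; BP_AI_Utility is an AI utility Blueprint that decides at random when a hunt starts and stops.
; A self-recalling delayed loop raises an appearance chance while idle or a disappearance chance while hunting, then rolls it against a random float.
; Each switch resets the opposite chance, and a stopped hunt adds an extra cooldown delay.
; HearNoise boosts the appearance chance, making hunts likelier after noise.
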(event Custom|Loop%20Percent
  (Utilities|FlowControl|Delay (Variables|Default|GetWaiting%20Second%20Loop))
  (if (Variables|Default|GetIs%20Hunting)
    (Disappearance|CalculDisappearancePercent)
    (bind _is_hunt_stopping (Disappearance|DetermineifHuntStop))
    (if _is_hunt_stopping
      (Utilities|FlowControl|Delay (Variables|Appearance|GetTime%20to%20Wait%20Between%20Two%20Apearance)))
    (else
      (Appearance|CalculAppearancePercent)
      (Appearance|DetermineifHuntStart)))
  (CallFunction|LoopPercent))

(event EventBeginPlay
  (Variables|Default|SetIs%20Hunting false)
  (CallFunction|LoopPercent))

(fn ConstructionScript)

(fn DetermineifHuntStop
  (if (> (Variables|Disappearance|GetDisappearance%20Percent) (Math|Random|RandomFloatinRange 0.0 1.0))
    (Variables|Default|SetIs%20Hunting false)
    (Variables|Appearance|SetAppearance%20Percent 0.0)
    (return true)
    (else
      (return false))))

(fn CalculDisappearancePercent
  (Variables|Disappearance|SetDisappearance%20Percent (+ (Variables|Disappearance|GetDisappearance%20Percent) (Variables|Disappearance|GetAmount%20Disappearance%20Percent))))

(fn CalculAppearancePercent
  (Variables|Appearance|SetAppearance%20Percent (+ (Variables|Appearance|GetAppearance%20Percent) (Variables|Appearance|GetAmount%20Appearance%20Percent))))

(fn DetermineifHuntStart
  (if (> (Variables|Appearance|GetAppearance%20Percent) (Math|Random|RandomFloatinRange 0.0 1.0))
    (Variables|Default|SetIs%20Hunting true)
    (Variables|Disappearance|SetDisappearance%20Percent 0.0)))

(fn HearNoise
  (Variables|Appearance|SetAppearance%20Percent (+ (Variables|Appearance|GetAppearance%20Percent) (Variables|Appearance|GetNoise%20Percent%20))))