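; BP_InteractibleDoor is an interactable, networked door that swings open away from or toward a side chosen by the player's position.
; Interaction flips a replicated toggle on the server, whose OnRep runs open/close through a gate open only while a first-person character overlaps the box.
; A dot product signs the door angle, and a timeline lerps yaw.
; The construction script configures mesh, widget, box, speed and interaction-area child actor.
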(event OnComponentBeginOverlap(Box)
  (params (OverlappedComponent :type Primitive%20Component%20Object%20Reference) (OtherActor :type Actor%20Object%20Reference) (OtherComp :type Primitive%20Component%20Object%20Reference) (OtherBodyIndex :type Integer) (bFromSweep :type Boolean) (SweepResult :type Hit%20Result%20Structure%20%28by%20ref%29))
  ;[1 0 0.4219] Open / Close door if player in the box
  (bind _asbp_first_person_character (Utilities|Casting|CastToBP_FirstPersonCharacter OtherActor))
  (Variables|Components|SetChar%20Ref _asbp_first_person_character)
  (Utilities|FlowControl|Gate true) ; enters at Open
)

(event OnComponentEndOverlap(Box)
  (params (OverlappedComponent :type Primitive%20Component%20Object%20Reference) (OtherActor :type Actor%20Object%20Reference) (OtherComp :type Primitive%20Component%20Object%20Reference) (OtherBodyIndex :type Integer))
  ;[1 0 0.4219] Open / Close door if player in the box
  (Utilities|Casting|CastToBP_FirstPersonCharacter OtherActor)
  (Utilities|FlowControl|Gate true) ; enters at Close
)

(event Custom|Interract
  ;[1 0 0.4219] Open / Close door if player in the box
  (Utilities|FlowControl|Gate true
    (:Exit
      ;[1 0.7266 0] If door is close Open the door depending on the player looking direction and door angle
      (if (not (Variables|Door|GetisOpened?))
        (Utilities|SetDirectedAngle (Variables|Components|GetChar%20Ref))
        (Variables|Door|SetisOpened? true)
        (bind _door_track (Timeline|OpenCloseDoorT Play)
          (:Update
            (Transformation|SetRelativeRotation (Variables|Default|GetDoor) (Math|Rotator|MakeRotator 0.0 0.0 (Math|Float|Lerp (Variables|Door|GetCloseDoor) (Variables|Door|GetDirectedAngle) _door_track)) false false)))
        (else
          (Variables|Door|SetisOpened? false)
          (Timeline|OpenCloseDoorT Reverse))))))

(event Custom|InteractOnServer
  ;[0 1 0.2031] Enable Interaction
  (Variables|Default|SetInteractToggle (not (Variables|Default|GetInteractToggle))))

(event EventBeginPlay
  (Development|PrintString (Utilities|String|Append "Yaw = " (Utilities|String|ToString(Float) (Variables|Door|GetCloseDoor))))
  (Development|PrintString (Utilities|String|Append "Door Angle = " (Utilities|String|ToString(Float) (Variables|Door|GetDoorAngle)))))

(event EventInterfaceInteract
  ;[0 1 0.2031] Enable Interaction
  (CallFunction|InteractonServer))

(event EventInterfaceToggleFocus
  (params (Focus :type Boolean))
  ;[0 1 0.2031] Enable Interaction
  (Rendering|SetRenderCustomDepth (Variables|Default|GetDoor) Focus))

(fn ConstructionScript
  (bind _door (Variables|Default|GetDoor))
  (bind _widget (Variables|Default|GetWidget))
  (bind _box (Variables|Default|GetBox))
  (Utilities|FlowControl|Sequence
    (:then_0
      ;[0 1 0.9063] Set Static Mesh
      (Components|StaticMesh|SetStaticMesh _door (Variables|InitMesh|GetBasicMesh))
      (Transformation|SetRelativeLocationAndRotation _door (Variables|InitMesh|GetMesh%20Location) (Variables|InitMesh|GetMesh%20Rotation) false false))
    (:then_1
      ;[0 1 0.9062] Set Widget Location
      (Transformation|SetRelativeLocation _widget (+ (Variables|/Script/Engine.SceneComponent|GetRelativeLocation _widget) (Variables|InitBox|GetWidget%20Location)) false false))
    (:then_2
      ;[0 1 0.9062] Set Child Actor Mesh
      (bind _asbp_interaction_area_custom_shape (Utilities|Casting|CastToBP_InteractionArea_Custom_Shape (Variables|/Script/Engine.ChildActorComponent|GetChildActor (Variables|Default|GetChildActor))))
      (Variables|/Game/Interaction/InteractionArea/BP_InteractionArea_Master.BP_InteractionArea_Master_C|SetInteractDuration _asbp_interaction_area_custom_shape (Variables|InitInteraction|GetInteract%20Duration))
      (Components|StaticMesh|SetStaticMesh (Variables|/Game/Interaction/InteractionArea/BP_InteractionArea_Custom_Shape.BP_InteractionArea_Custom_Shape_C|GetShape _asbp_interaction_area_custom_shape) (Variables|InitMesh|GetBasicMesh)))
    (:then_3
      ;[0 1 0.9062] Set Door Speed and Angle
      ;;[1 0.09375 0] Speed
      (Components|Timeline|SetPlayRate (Variables|Default|GetOpenCloseDoorT) (/ 1.0 (Variables|InitInteraction|GetOCDuration))))
    (:then_4
      ;[0 1 0.9062] Set Box Location
      (Transformation|SetRelativeLocation _box (Variables|InitBox|GetBox%20Location) false false)
      (Transformation|SetRelativeScale3D _box (Variables|InitBox|GetBox%20Colision%20Scale)))
    (:then_5
      (Variables|Door|SetCloseDoor (.yaw (Transformation|GetSocketRotation (Variables|Default|GetDoor) "None"))))))

(fn OnRepInteractToggle
  (CallFunction|Interract))

(fn GetInteractionWidgetRef
  (return (Variables|Default|GetWidget)))