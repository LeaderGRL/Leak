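; BP_NPC is an enemy NPC that takes damage through a HitEnemy event and dies at zero health.
; On BeginPlay it caches the first-person player character, all AI utility actors and all spawner managers.
; On death it calls SplashCAM on the player, destroys itself and sets IsDispawning on every spawner manager.
; Hits and kills are reported with on-screen debug prints.
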(event EventHitEnemy
  (params (Damage :type Float%20%28double-precision%29))
  (bind _output_get (Variables|Default|SetHealth (- (Variables|Default|GetHealth) Damage)))
  (if (<= _output_get 0.0)
    (Development|PrintString "Enemy Killed" true true "(R=1.000000,G=0.000000,B=0.000000,A=1.000000)")
    (Default|SplashCAM (Variables|Default|GetChara%20REF))
    (Actor|DestroyActor)
    (for _array_element (Variables|Default|GetSpawnerREF)
      (Variables|/Game/Leak/Blueprints/AI_Utility/BP_SpawnerManager.BP_SpawnerManager_C|SetIsDispawning _array_element true))
    (else
      (Development|PrintString (Utilities|String|ToString(Float) _output_get) true true "(R=1.000000,G=0.000000,B=0.000000,A=1.000000)"))))

(event EventBeginPlay
  (bind _asbp_first_person_character (Utilities|Casting|CastToBP_FirstPersonCharacter (Game|GetPlayerCharacter 0)))
  (Variables|Default|SetChara%20REF _asbp_first_person_character)
  (bind _outactors (Actor|GetAllActorsOfClass "/Game/Leak/Blueprints/AI_Utility/BP_AI_Utility_V2.BP_AI_Utility_V2_C"))
  (Variables|Default|SetAI%20Utility%20REF _outactors)
  (bind _outactors_2 (Actor|GetAllActorsOfClass "/Game/Leak/Blueprints/AI_Utility/BP_SpawnerManager.BP_SpawnerManager_C"))
  (Variables|Default|SetSpawnerREF _outactors_2))

(fn ConstructionScript)