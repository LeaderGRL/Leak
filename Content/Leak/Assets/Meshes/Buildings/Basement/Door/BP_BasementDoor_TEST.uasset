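; Sliding double basement door that opens when something overlaps its Box trigger and closes when the overlap ends.
; A timeline lerps both panels between stored positions, playing to open and reversing to close, with both blocked while IsLock is set.
; Lock, unlock and light events set that flag or swap the frame material between light, red and black.
; ResetDoor uses a second timeline to move the panels back, ignoring the lock.
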(event OnComponentBeginOverlap(Box)
  (params (OverlappedComponent :type Primitive%20Component%20Object%20Reference) (OtherActor :type Actor%20Object%20Reference) (OtherComp :type Primitive%20Component%20Object%20Reference) (OtherBodyIndex :type Integer) (bFromSweep :type Boolean) (SweepResult :type Hit%20Result%20Structure%20%28by%20ref%29))
  (CallFunction|OpenDoor))

(event OnComponentEndOverlap(Box)
  (params (OverlappedComponent :type Primitive%20Component%20Object%20Reference) (OtherActor :type Actor%20Object%20Reference) (OtherComp :type Primitive%20Component%20Object%20Reference) (OtherBodyIndex :type Integer))
  (CallFunction|CloseDoor))

(event Custom|LockDoor
  (Variables|Default|SetIsLock true)
  (if (Variables|Default|GetIsOpenning)
    (CallFunction|CloseDoor)))

(event Custom|unlockDoor
  (Variables|Default|SetIsLock false)
  (Rendering|Material|SetMaterial (Variables|Default|GetSM_BasementDoor_Cadre) 1 "/Game/Leak/Assets/Meshes/Buildings/Basement/Door/MI_BasementDoor_Light.MI_BasementDoor_Light"))

(event Custom|CloseDoor
  (if (not (Variables|Default|GetIsLock))
    (bind _newtrack_0 (Timeline|Timeline Reverse)
      (:Update
        (Utilities|FlowControl|Sequence
          (:then_0
            (Transformation|SetRelativeLocation (Variables|Default|GetSM_BasementDoor_Right) (Math|Vector|Lerp(Vector) (Variables|Default|GetCurrentRight) (Variables|Default|GetNewRight) _newtrack_0) false false))
          (:then_1
            (Transformation|SetRelativeLocation (Variables|Default|GetSM_BasementDoor_Left) (Math|Vector|Lerp(Vector) (Variables|Default|GetCurrentLeft) (Variables|Default|GetNewLeft) _newtrack_0) false false))))
      (:Finished
        (Variables|Default|SetIsOpenning false)))))

(event Custom|OpenDoor
  (if (not (Variables|Default|GetIsLock))
    (Variables|Default|SetIsOpenning true)
    (bind _newtrack_0 (Timeline|Timeline Play)
      (:Update
        (Utilities|FlowControl|Sequence
          (:then_0
            (Transformation|SetRelativeLocation (Variables|Default|GetSM_BasementDoor_Right) (Math|Vector|Lerp(Vector) (Variables|Default|GetCurrentRight) (Variables|Default|GetNewRight) _newtrack_0) false false))
          (:then_1
            (Transformation|SetRelativeLocation (Variables|Default|GetSM_BasementDoor_Left) (Math|Vector|Lerp(Vector) (Variables|Default|GetCurrentLeft) (Variables|Default|GetNewLeft) _newtrack_0) false false))))
      (:Finished
        (Variables|Default|SetIsOpenning false)))))

(event Custom|Activate%20light
  (Rendering|Material|SetMaterial (Variables|Default|GetSM_BasementDoor_Cadre) 1 "/Game/Leak/Assets/Materials/Buildings/Basement/MI_Basement_Door_Red.MI_Basement_Door_Red"))

(event Custom|ResetDoor
  (bind _newtrack_0 (Timeline|Timeline_0 Play)
    (:Update
      (Utilities|FlowControl|Sequence
        (:then_0
          (Transformation|SetRelativeLocation (Variables|Default|GetSM_BasementDoor_Right) (Math|Vector|Lerp(Vector) (Variables|Default|GetNewRight) (Variables|Default|GetCurrentRight) _newtrack_0) false false))
        (:then_1
          (Transformation|SetRelativeLocation (Variables|Default|GetSM_BasementDoor_Left) (Math|Vector|Lerp(Vector) (Variables|Default|GetNewLeft) (Variables|Default|GetCurrentLeft) _newtrack_0) false false))))))

(event Custom|Turn%20Off%20Light
  (Rendering|Material|SetMaterial (Variables|Default|GetSM_BasementDoor_Cadre) 1 "/Game/Leak/Assets/Materials/Specials/M_Black.M_Black"))

(event Custom|Active%20Red%20Light
  (Rendering|Material|SetMaterial (Variables|Default|GetSM_BasementDoor_Cadre) 1 "/Game/Leak/Assets/Materials/Buildings/Basement/MI_Basement_Door_Red.MI_Basement_Door_Red"))

(fn ConstructionScript)