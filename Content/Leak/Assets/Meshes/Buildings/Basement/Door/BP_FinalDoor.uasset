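; Final laboratory double door that the player opens with the interact input to trigger the ending cinematic.
; Entering UnlockBox moves the interaction Box into place, whose overlap shows a prompt and enables input.
; Interact toggles a timeline that slides both panels apart or back.
; Opening also removes the point light, spins two repositioned spotlights on a second timeline, and adds the ending widget through a two-second Delay driven by that timeline's Update.
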(event OnComponentBeginOverlap(UnlockBox)
  (params (OverlappedComponent :type Primitive%20Component%20Object%20Reference) (OtherActor :type Actor%20Object%20Reference) (OtherComp :type Primitive%20Component%20Object%20Reference) (OtherBodyIndex :type Integer) (bFromSweep :type Boolean) (SweepResult :type Hit%20Result%20Structure%20%28by%20ref%29))
  (Utilities|Casting|CastToBP_FirstPersonCharacter OtherActor)
  (Transformation|SetRelativeLocation (Variables|Default|GetBox) "235.000000,0.000000,100.000000" false false))

(event OnComponentBeginOverlap(Box)
  (params (OverlappedComponent :type Primitive%20Component%20Object%20Reference) (OtherActor :type Actor%20Object%20Reference) (OtherComp :type Primitive%20Component%20Object%20Reference) (OtherBodyIndex :type Integer) (bFromSweep :type Boolean) (SweepResult :type Hit%20Result%20Structure%20%28by%20ref%29))
  (bind _asbp_first_person_character (Utilities|Casting|CastToBP_FirstPersonCharacter OtherActor))
  (Variables|Default|SetCharaREF _asbp_first_person_character)
  (bind _returnvalue (UserInterface|CreateWidget "/Game/Leak/Blueprints/Interaction/WB_NewInteraction_E.WB_NewInteraction_E_C"))
  (UserInterface|Viewport|AddtoViewport _returnvalue 0)
  (Input|EnableInput (Game|GetPlayerController 0))
  (Utilities|FlowControl|Gate true) ; enters at Open
)

(event OnComponentEndOverlap(Box)
  (params (OverlappedComponent :type Primitive%20Component%20Object%20Reference) (OtherActor :type Actor%20Object%20Reference) (OtherComp :type Primitive%20Component%20Object%20Reference) (OtherBodyIndex :type Integer))
  (Utilities|Casting|CastToBP_FirstPersonCharacter OtherActor)
  (bind _foundwidgets (Widget|GetAllWidgetsOfClass "/Game/Leak/Blueprints/Interaction/WB_NewInteraction_E.WB_NewInteraction_E_C" true))
  (Widget|RemovefromParent _foundwidgets)
  (Input|DisableInput (Game|GetPlayerController 0))
  (Utilities|FlowControl|Gate true) ; enters at Close
)

(event Custom|OpenDoor
  (bind _close_angle (Variables|Default|GetClose%20Angle))
  (Variables|Default|SetIsOpened? true)
  (bind _doortrack (Timeline|Timeline PlayFromStart)
    (:Update
      (Transformation|SetRelativeLocation (Variables|Default|GetSM_Door_Labo_Door_Right) (Math|Vector|MakeVector (Math|Float|Lerp _close_angle (Variables|Default|GetOpen%20Angle) _doortrack) 0.0 0.0) false false)
      (Transformation|SetRelativeLocation (Variables|Default|GetSM_Door_Labo_Door_Left) (Math|Vector|MakeVector (Math|Float|Lerp _close_angle -2e+02 _doortrack) 0.0 0.0) false false))))

(event Custom|CloseDoor
  (bind _close_angle (Variables|Default|GetClose%20Angle))
  (Variables|Default|SetIsOpened? false)
  (bind _doortrack (Timeline|Timeline ReverseFromEnd)
    (:Update
      (Transformation|SetRelativeLocation (Variables|Default|GetSM_Door_Labo_Door_Right) (Math|Vector|MakeVector (Math|Float|Lerp _close_angle (Variables|Default|GetOpen%20Angle) _doortrack) 0.0 0.0) false false)
      (Transformation|SetRelativeLocation (Variables|Default|GetSM_Door_Labo_Door_Left) (Math|Vector|MakeVector (Math|Float|Lerp _close_angle -2e+02 _doortrack) 0.0 0.0) false false))))

(event Input|EnhancedActionEvents|EnhancedInputActionIA_Interact
  (params (ActionValue :type Boolean) (ElapsedSeconds :type Float%20%28double-precision%29) (TriggeredSeconds :type Float%20%28double-precision%29) (InputAction :type Input%20Action%20Object%20Reference :default "/Game/Leak/Inputs/Actions/IA_Interact.IA_Interact"))
  (:Started
    (if (Variables|Default|GetIsOpened?)
      (CallFunction|CloseDoor)
      (else
        (CallFunction|OpenDoor)
        (Transformation|SetRelativeLocation (Variables|Default|GetSpotLight) "0.000000,-75.000000,250.000000" false false)
        (Components|DestroyComponent (Variables|Default|GetPointLight))
        (bind _newtrack_0 (Timeline|Timeline_0 Play)
          (:Update
            (Transformation|SetRelativeRotation (Variables|Default|GetSpotLight) (Math|Rotator|MakeRotator 0.0 0.0 (Math|Float|Lerp 0.0 3.6e+02 _newtrack_0)) false false)
            (Transformation|SetRelativeRotation (Variables|Default|GetSpotLight1) (Math|Rotator|MakeRotator 0.0 0.0 (Math|Float|Lerp -1.8e+02 1.8e+02 _newtrack_0)) false false)
            (Utilities|FlowControl|Delay 2.0)
            (bind _returnvalue (UserInterface|CreateWidget "/Game/Leak/Cinematic/WB_Cinematic_Fin.WB_Cinematic_Fin_C"))
            (UserInterface|Viewport|AddtoViewport _returnvalue 0)))))))

(event EventBeginPlay)

(fn ConstructionScript)