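; Basement button that unlocks the doors tagged ToUnlockB and spawns a behavior-tree NPC at a fixed location when pressed.
; Entering UnclockBox arms it, so overlapping Box then shows an interaction widget and enables input until the player leaves.
; Interact plays a timeline sliding the button, calling UnlockDoor on doors cached at BeginPlay and teleporting Box on every update.
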(event OnComponentBeginOverlap(Box)
  (params (OverlappedComponent :type Primitive%20Component%20Object%20Reference) (OtherActor :type Actor%20Object%20Reference) (OtherComp :type Primitive%20Component%20Object%20Reference) (OtherBodyIndex :type Integer) (bFromSweep :type Boolean) (SweepResult :type Hit%20Result%20Structure%20%28by%20ref%29))
  (if (Variables|Default|GetUnlockBox)
    (bind _asbp_first_person_character (Utilities|Casting|CastToBP_FirstPersonCharacter OtherActor))
    (Variables|Default|SetChara%20REF _asbp_first_person_character)
    (bind _returnvalue (UserInterface|CreateWidget "/Game/Leak/Blueprints/Interaction/WB_NewInteraction.WB_NewInteraction_C"))
    (UserInterface|Viewport|AddtoViewport _returnvalue 0)
    (Input|EnableInput (Game|GetPlayerController 0))))

(event OnComponentEndOverlap(Box)
  (params (OverlappedComponent :type Primitive%20Component%20Object%20Reference) (OtherActor :type Actor%20Object%20Reference) (OtherComp :type Primitive%20Component%20Object%20Reference) (OtherBodyIndex :type Integer))
  (Utilities|Casting|CastToBP_FirstPersonCharacter OtherActor)
  (bind _foundwidgets (Widget|GetAllWidgetsOfClass "/Game/Leak/Blueprints/Interaction/WB_NewInteraction.WB_NewInteraction_C" true))
  (Widget|RemovefromParent _foundwidgets)
  (Input|DisableInput (Game|GetPlayerController 0)))

(event OnComponentBeginOverlap(UnclockBox)
  (params (OverlappedComponent :type Primitive%20Component%20Object%20Reference) (OtherActor :type Actor%20Object%20Reference) (OtherComp :type Primitive%20Component%20Object%20Reference) (OtherBodyIndex :type Integer) (bFromSweep :type Boolean) (SweepResult :type Hit%20Result%20Structure%20%28by%20ref%29))
  (Utilities|Casting|CastToBP_FirstPersonCharacter OtherActor)
  (Variables|Default|SetUnlockBox true))

(event Input|EnhancedActionEvents|EnhancedInputActionIA_Interact
  (params (ActionValue :type Boolean) (ElapsedSeconds :type Float%20%28double-precision%29) (TriggeredSeconds :type Float%20%28double-precision%29) (InputAction :type Input%20Action%20Object%20Reference :default "/Game/Leak/Inputs/Actions/IA_Interact.IA_Interact"))
  (Utilities|Casting|CastToBP_FirstPersonCharacter (Game|GetPlayerCharacter 0))
  (Utilities|FlowControl|Sequence
    (:then_0
      (bind _newtrack_0 (Timeline|Timeline Play)
        (:Update
          (Transformation|SetRelativeLocation (Variables|Default|GetButton) (Math|Vector|Lerp(Vector) "0.000000,67.000000,0.000000" "0.000000,27.000000,0.000000" _newtrack_0) false false)
          (for _array_element (Variables|Default|GetOut%20Actors)
            (Default|UnlockDoor _array_element)
            (Transformation|SetRelativeLocation (Variables|Default|GetBox) "17.000000,60.000000,-275.000000" false true)))))
    (:then_1
      (AI|SpawnAIFromClass "/Game/Leak/AI/BP_NPC.BP_NPC_C" "/Game/Leak/AI/BT_NPC.BT_NPC" "-950.000000,-700.000000,-500.000000" "0, 0, 0" false 0))))

(event EventBeginPlay
  (bind _outactors (Actor|GetAllActorsOfClasswithTag "/Game/Leak/Assets/Meshes/Buildings/Basement/Door/BP_BasementDoor_TEST.BP_BasementDoor_TEST_C" "ToUnlockB"))
  (Variables|Default|SetOut%20Actors _outactors))

(fn ConstructionScript)