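; BP_BasementDoor is a double basement door that slides open when something overlaps its Box trigger and closes when an overlap ends.
; A Timeline plays on begin overlap and reverses on end overlap, with no filter on the overlapping actor.
; Its track lerps the relative locations of the left and right door meshes between Current and New position variables, which the graphs never set.
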(event OnComponentBeginOverlap(Box)
  (params (OverlappedComponent :type Primitive%20Component%20Object%20Reference) (OtherActor :type Actor%20Object%20Reference) (OtherComp :type Primitive%20Component%20Object%20Reference) (OtherBodyIndex :type Integer) (bFromSweep :type Boolean) (SweepResult :type Hit%20Result%20Structure%20%28by%20ref%29))
  (bind _newtrack_0 (Timeline|Timeline Play)
    (:Update
      (Utilities|FlowControl|Sequence
        (:then_0
          (Transformation|SetRelativeLocation (Variables|Default|GetSM_BasementDoor_Right) (Math|Vector|Lerp(Vector) (Variables|Default|GetCurrentRight) (Variables|Default|GetNewRight) _newtrack_0) false false))
        (:then_1
          (Transformation|SetRelativeLocation (Variables|Default|GetSM_BasementDoor_Left) (Math|Vector|Lerp(Vector) (Variables|Default|GetCurrentLeft) (Variables|Default|GetNewLeft) _newtrack_0) false false))))))

(event OnComponentEndOverlap(Box)
  (params (OverlappedComponent :type Primitive%20Component%20Object%20Reference) (OtherActor :type Actor%20Object%20Reference) (OtherComp :type Primitive%20Component%20Object%20Reference) (OtherBodyIndex :type Integer))
  (bind _newtrack_0 (Timeline|Timeline Reverse)
    (:Update
      (Utilities|FlowControl|Sequence
        (:then_0
          (Transformation|SetRelativeLocation (Variables|Default|GetSM_BasementDoor_Right) (Math|Vector|Lerp(Vector) (Variables|Default|GetCurrentRight) (Variables|Default|GetNewRight) _newtrack_0) false false))
        (:then_1
          (Transformation|SetRelativeLocation (Variables|Default|GetSM_BasementDoor_Left) (Math|Vector|Lerp(Vector) (Variables|Default|GetCurrentLeft) (Variables|Default|GetNewLeft) _newtrack_0) false false))))))

(fn ConstructionScript)