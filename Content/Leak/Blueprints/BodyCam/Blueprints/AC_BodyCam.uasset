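; Actor component that gives the character's first-person view a bodycam feel through camera shake and a moving vignette.
; Each tick it starts an idle, walk or run camera shake chosen by character speed.
; Clamped, smoothed camera rotation deltas drive the VignetteOffset parameter in MPC_Vignette, making the vignette lag with look movement.
; At walk speed or above, interpolated random values also drive VignetteShake for jitter.
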(event Custom|Camera%20Shake%20Event
  (bind _returnvalue (Game|GetPlayerController 0))
  (bind _charref (Variables|Default|GetCharRef))
  (bind _shakescale (Variables|Default|GetShakeScale))
  (bind _returnvalue_2 (Transformation|GetVelocity _charref))
  (bind _returnvalue_3 (Math|Vector|VectorLength _returnvalue_2))
  ;[0 0.6016 1] Camera Shake
  (if (< _returnvalue_3 (Variables|/Game/Leak/Blueprints/Character/BP_FirstPersonCharacter.BP_FirstPersonCharacter_C|GetWalk%20Speed _charref))
    (Game|Feedback|ClientStartCameraShake _returnvalue "/Game/Leak/Blueprints/BodyCam/Camera_Shake_Idle.Camera_Shake_Idle_C" _shakescale "CameraLocal" "0, 0, 0")
    (elif (> _returnvalue_3 (Variables|/Game/Leak/Blueprints/Character/BP_FirstPersonCharacter.BP_FirstPersonCharacter_C|GetSprint%20Speed _charref))
      (Game|Feedback|ClientStartCameraShake _returnvalue "/Game/Leak/Blueprints/BodyCam/Camera_Shake_Run.Camera_Shake_Run_C" _shakescale "CameraLocal" "0, 0, 0")
      (else
        (Game|Feedback|ClientStartCameraShake _returnvalue "/Game/Leak/Blueprints/BodyCam/Camera_Shake_Walk.Camera_Shake_Walk_C" _shakescale "CameraLocal" "0, 0, 0")))))

(event EventTick
  (params (DeltaSeconds :type Float%20%28single-precision%29))
  (bind _returnvalue (Utilities|Time|GetWorldDeltaSeconds))
  (bind _returnvalue_2 (Utilities|Time|GetWorldDeltaSeconds))
  (bind _returnvalue_3 (Utilities|Time|GetWorldDeltaSeconds))
  (bind _returnvalue_4 (Utilities|Time|GetWorldDeltaSeconds))
  (bind _charref (Variables|Default|GetCharRef))
  (bind _yawrateminmax (Variables|Default|GetYawRateMinMax))
  (bind _pitchrateminmax (Variables|Default|GetPitchRateMinMax))
  (bind _charref_2 (Variables|Default|GetCharRef))
  (bind _firstpersoncamera (Variables|/Game/Leak/Blueprints/Character/BP_FirstPersonCharacter.BP_FirstPersonCharacter_C|GetFirstPersonCamera _charref))
  (bind _returnvalue_5 (Transformation|GetWorldRotation _firstpersoncamera))
  (bind (_roll _pitch _yaw) (Math|Rotator|BreakRotator _returnvalue_5))
  ;[1 0.4453 0] Vignette Wobble
  (Utilities|FlowControl|Sequence
    (:then_0
      (CallFunction|CameraShakeEvent))
    (:then_1
      (Variables|Default|SetPitchRate (Math|Float|Clamp(Float) (+ (Variables|Default|GetPitchRate) (- _pitch (.pitch (Variables|Default|GetCamRotator)))) (* _pitchrateminmax -1.0) _pitchrateminmax))
      (Variables|Default|SetYawRate (Math|Float|Clamp(Float) (+ (Variables|Default|GetYawRate) (- _yaw (.yaw (Variables|Default|GetCamRotator)))) (* _yawrateminmax -1.0) _yawrateminmax))
      (Variables|Default|SetCamRotator _returnvalue_5)
      (bind _output_get (Variables|Default|SetPitch%20Vignette%20Offset (Math|Interpolation|FInterpTo (Variables|Default|GetPitch%20Vignette%20Offset) (Variables|Default|GetPitchRate) _returnvalue 1e+01)))
      (bind _output_get_2 (Variables|Default|SetYaw%20Vignette%20Offset (Math|Interpolation|FInterpTo (Variables|Default|GetYaw%20Vignette%20Offset) (Variables|Default|GetYawRate) _returnvalue 1e+01)))
      (Rendering|Material|SetVectorParameterValue "/Game/Leak/Blueprints/BodyCam/PostProcess_Materials/MPC_Vignette.MPC_Vignette" "VignetteOffset" (Utilities|Struct|MakeLinearColor _output_get_2 _output_get 0.0 1.0) :!class /Script/Engine.KismetMaterialLibrary)
      (Variables|Default|SetYawRate (Math|Interpolation|FInterpTo (Variables|Default|GetYawRate) 0.0 (Utilities|Time|GetWorldDeltaSeconds) 15.0))
      (Variables|Default|SetPitchRate (Math|Interpolation|FInterpTo (Variables|Default|GetPitchRate) 0.0 (Utilities|Time|GetWorldDeltaSeconds) 15.0)))
    (:then_2
      (if (>= (Math|Vector|VectorLength (Transformation|GetVelocity _charref_2)) (Variables|/Game/Leak/Blueprints/Character/BP_FirstPersonCharacter.BP_FirstPersonCharacter_C|GetWalk%20Speed _charref_2))
        ;[0.125 1 0] Vignette Shake
        (Variables|Default|SetPitch%20Shake (Math|Interpolation|FInterpTo (Variables|Default|GetPitch%20Shake) (Math|Random|RandomFloatinRange -1e+01 1e+01) _returnvalue_4 3.0))
        (Variables|Default|SetYaw%20Shake (Math|Interpolation|FInterpTo (Variables|Default|GetYaw%20Shake) (Math|Random|RandomFloatinRange -1e+01 1e+01) _returnvalue_4 3.0))
        (bind _output_get_3 (Variables|Default|SetPitch%20Vignette%20Shake (Math|Interpolation|FInterpTo (Variables|Default|GetPitch%20Vignette%20Shake) (Variables|Default|GetPitch%20Shake) _returnvalue_2 2e+01)))
        (bind _output_get_4 (Variables|Default|SetYaw%20Vignette%20Shake (Math|Interpolation|FInterpTo (Variables|Default|GetYaw%20Vignette%20Shake) (Variables|Default|GetYaw%20Shake) _returnvalue_2 2e+01)))
        (Rendering|Material|SetVectorParameterValue "/Game/Leak/Blueprints/BodyCam/PostProcess_Materials/MPC_Vignette.MPC_Vignette" "VignetteShake" (Utilities|Struct|MakeLinearColor _output_get_4 _output_get_3 0.0 1.0) :!class /Script/Engine.KismetMaterialLibrary)
        (Variables|Default|SetPitch%20Vignette%20Shake (Math|Interpolation|FInterpTo (Variables|Default|GetPitch%20Shake) 0.0 _returnvalue_3 2e+01))
        (Variables|Default|SetYaw%20Vignette%20Shake (Math|Interpolation|FInterpTo (Variables|Default|GetYaw%20Shake) 0.0 _returnvalue_3 2e+01))))))