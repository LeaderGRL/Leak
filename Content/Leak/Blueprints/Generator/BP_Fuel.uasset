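; BP_Fuel is an interactable fuel item that the first-person player picks up to use with the generator.
; On interact it attaches to the character's FuelGripPoint socket, flags itself as attached and disables its mesh collision.
; It then finds the BP_Generator in the level and changes that generator's interaction duration, while the toggle-focus event switches off the fuel's custom-depth highlight.
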(event Custom|Interact
  (bind _asbp_first_person_character (Utilities|Casting|CastToBP_FirstPersonCharacter (Game|GetPlayerCharacter 0)))
  (bind _returnvalue (Transformation|AttachComponentToComponent (Variables|/Game/Leak/Blueprints/Character/BP_FirstPersonCharacter.BP_FirstPersonCharacter_C|GetFirstPersonMesh _asbp_first_person_character) "FuelGripPoint" "SnapToTarget" "SnapToTarget" "KeepRelative" true))
  (if _returnvalue
    (Variables|Default|SetFuelAttached true)
    (Collision|SetCollisionEnabled (Variables|Default|GetFuel) "NoCollision")
    (bind _returnvalue_2 (Actor|GetActorOfClass "/Game/Leak/Blueprints/Generator/BP_Generator.BP_Generator_C"))
    (Default|ChangeInterractDuration _returnvalue_2 4.0)
    (else
      (Development|PrintString "Not Snapped"))))

(event EventInterfaceToggleFocus
  (params (Focus :type Boolean))
  (Rendering|SetRenderCustomDepth (Variables|Default|GetFuel) false))

(event EventInterfaceInteract
  (CallFunction|Interact))

(fn ConstructionScript)