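; Basement generator that the player powers with carried fuel to switch on lights and change door states.
; Overlapping the box, once a temporary unlock volume is exited, shows a prompt and enables input.
; Interacting consumes fuel and chains battery and lever timelines through Delays in their Update pins.
; These drive doors and lamps gathered on BeginPlay by class or tag, plus turbine spin, idle sound and red-to-green indicator.
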(event OnComponentBeginOverlap(Box)
  (params (OverlappedComponent :type Primitive%20Component%20Object%20Reference) (OtherActor :type Actor%20Object%20Reference) (OtherComp :type Primitive%20Component%20Object%20Reference) (OtherBodyIndex :type Integer) (bFromSweep :type Boolean) (SweepResult :type Hit%20Result%20Structure%20%28by%20ref%29))
  (if (Variables|Default|GetUnlock%20Box)
    (bind _asbp_first_person_character (Utilities|Casting|CastToBP_FirstPersonCharacter OtherActor))
    (Variables|Default|SetChara%20REF _asbp_first_person_character)
    (bind _returnvalue (UserInterface|CreateWidget "/Game/Leak/Blueprints/Interaction/WB_NewInteraction.WB_NewInteraction_C"))
    (UserInterface|Viewport|AddtoViewport _returnvalue 0)
    (Input|EnableInput (Game|GetPlayerController 0))))

(event OnComponentEndOverlap(UnlockBox)
  (params (OverlappedComponent :type Primitive%20Component%20Object%20Reference) (OtherActor :type Actor%20Object%20Reference) (OtherComp :type Primitive%20Component%20Object%20Reference) (OtherBodyIndex :type Integer))
  ;[1 1 1] TEMPORAIRE
  (Utilities|Casting|CastToBP_FirstPersonCharacter OtherActor)
  (Variables|Default|SetUnlock%20Box true))

(event OnComponentEndOverlap(Box)
  (params (OverlappedComponent :type Primitive%20Component%20Object%20Reference) (OtherActor :type Actor%20Object%20Reference) (OtherComp :type Primitive%20Component%20Object%20Reference) (OtherBodyIndex :type Integer))
  (Utilities|Casting|CastToBP_FirstPersonCharacter OtherActor)
  (bind _foundwidgets (Widget|GetAllWidgetsOfClass "/Game/Leak/Blueprints/Interaction/WB_NewInteraction.WB_NewInteraction_C" true))
  (Widget|RemovefromParent _foundwidgets)
  (Input|DisableInput (Game|GetPlayerController 0)))

(event Custom|Interact
  (bind _sm_generator_battery (Variables|Default|GetSM_Generator_Battery))
  (bind _asbp_first_person_character (Utilities|Casting|CastToBP_FirstPersonCharacter (Game|GetPlayerCharacter 0)))
  (if (Variables|/Game/Leak/Blueprints/Character/BP_FirstPersonCharacter.BP_FirstPersonCharacter_C|GetHasFuel _asbp_first_person_character)
    (Variables|Default|Setpower true)
    (Variables|/Game/Leak/Blueprints/Character/BP_FirstPersonCharacter.BP_FirstPersonCharacter_C|SetHasFuel _asbp_first_person_character false)
    (Development|PrintString "Fuel loaded")
    (Utilities|FlowControl|Sequence
      (:then_0
        (Transformation|SetRelativeLocation (Variables|Default|GetBox) "-109.000000,-85.000000,-130.000000" false false))
      (:then_1
        (Development|SetHiddeninGame _sm_generator_battery false false)
        (bind _newtrack_0 (Timeline|Fuel Play)
          (:Update
            (Transformation|SetRelativeLocation _sm_generator_battery (Math|Vector|Lerp(Vector) "-82.000000,-104.000000,82.000000" "-42.000000,-104.000000,82.000000" _newtrack_0) true false)
            (Transformation|SetRelativeRotation _sm_generator_battery (Math|Rotator|Lerp(Rotator) "0, 0, 0" "0.000000,0.000000,120.000000" _newtrack_0) false false)
            (Utilities|FlowControl|Delay 1.0)
            (bind _levier_rotation (Timeline|Timeline Play)
              (:Update
                (Transformation|SetRelativeRotation (Variables|Default|GetTEST) (Math|Rotator|Lerp(Rotator) "0, 0, 0" "90.000000,0.000000,0.000000" _levier_rotation) false false)
                (Utilities|FlowControl|Delay 1.0)
                (Utilities|FlowControl|Sequence
                  (:then_0
                    (for _array_element (Variables|Default|GetDoorsToUnlock)
                      (Default|UnlockDoor _array_element)
                      (Default|ActivateLight _array_element)))
                  (:then_1
                    (for _array_element_2 (Variables|Default|GetDoorsToLock)
                      (Default|LockDoor _array_element_2)
                      (Default|ActivateLight _array_element_2)))
                  (:then_2
                    (for _array_element_3 (Variables|Default|GetBasementLampA)
                      (Default|ActivateLight _array_element_3)))
                  (:then_3
                    (for _array_element_4 (Variables|Default|GetBasementLampB)
                      (Default|ActivateLight _array_element_4)))
                  (:then_4
                    (for _array_element_5 (Variables|Default|GetBasementLampC)
                      (Default|ActivateLight _array_element_5)))
                  (:then_5
                    (for _array_element_6 (Variables|Default|GetDOORTEST)
                      (Default|ResetDoor _array_element_6)
                      (Default|ActivateLight _array_element_6)))
                  (:then_6
                    (for _array_element_7 (Variables|Default|GetA)
                      (Default|ActivateLight _array_element_7)))
                  (:then_7
                    (for _array_element_8 (Variables|Default|GetB)
                      (Default|ActivateLight _array_element_8)))
                  (:then_8
                    (bind _newtrack_0_2 (Timeline|Timeline_0 Play)
                      (:Update
                        (Transformation|SetRelativeRotation (Variables|Default|GetChildActorTurbine) (Math|Rotator|Lerp(Rotator) "0, 0, 0" "360.000000,0.000000,0.000000" _newtrack_0_2) false false))))
                  (:then_9
                    (Audio|PlaySoundatLocation "/Game/Leak/Assets/Audio/Generator/SC_Generator_Idle.SC_Generator_Idle" (Transformation|GetSocketLocation (Variables|Default|GetGenerator) "None") "0, 0, 0" 1.0 1.0 0.0 0 0 0 0))
                  (:then_10
                    (Rendering|SetVisibility (Variables|Default|GetRedLight) false false)
                    (Rendering|SetVisibility (Variables|Default|GetGreenLight) true false)))))))))
    (else
      (Audio|PlaySound2D "/Game/Leak/Assets/Audio/Flashlight/flashlight-on.flashlight-on" 1.0 1.0 0.0 0 0)
      (Development|PrintString "Need Fuel"))))

(event Input|EnhancedActionEvents|EnhancedInputActionIA_Interact
  (params (ActionValue :type Boolean) (ElapsedSeconds :type Float%20%28double-precision%29) (TriggeredSeconds :type Float%20%28double-precision%29) (InputAction :type Input%20Action%20Object%20Reference :default "/Game/Leak/Inputs/Actions/IA_Interact.IA_Interact"))
  (CallFunction|Interact))

(event EventBeginPlay
  (Utilities|FlowControl|Sequence
    (:then_0
      (bind _outactors (Actor|GetAllActorsOfClasswithTag "/Game/Leak/Assets/Meshes/Buildings/Basement/Door/BP_BasementDoor.BP_BasementDoor_C" "ToLock"))
      (Variables|Default|SetDoorsToLock _outactors))
    (:then_1
      (bind _outactors_2 (Actor|GetAllActorsOfClasswithTag "/Game/Leak/Assets/Meshes/Buildings/Basement/Door/BP_BasementDoor.BP_BasementDoor_C" "ToUnlock"))
      (Variables|Default|SetDoorsToUnlock _outactors_2))
    (:then_2
      (bind _outactors_3 (Actor|GetAllActorsOfClass "/Game/Leak/Blueprints/Light/BP_Basement_Lamp_A.BP_Basement_Lamp_A_C"))
      (Variables|Default|SetBasementLampA _outactors_3))
    (:then_3
      (bind _outactors_4 (Actor|GetAllActorsOfClass "/Game/Leak/Blueprints/Light/BP_Basement_Lamp_B.BP_Basement_Lamp_B_C"))
      (Variables|Default|SetBasementLampB _outactors_4))
    (:then_4
      (bind _outactors_5 (Actor|GetAllActorsOfClass "/Game/Leak/Blueprints/Light/BP_Basement_Lamp_C.BP_Basement_Lamp_C_C"))
      (Variables|Default|SetBasementLampC _outactors_5))
    (:then_5
      (bind _outactors_6 (Actor|GetAllActorsOfClasswithTag "/Game/Leak/Assets/Meshes/Buildings/Basement/Door/BP_BasementDoor_TEST.BP_BasementDoor_TEST_C" "ToLock"))
      (Variables|Default|SetDOORTEST _outactors_6))
    (:then_6
      (bind _outactors_7 (Actor|GetAllActorsOfClass "/Game/Leak/Assets/Meshes/Buildings/Basement/Door/BP_BasementDoor.BP_BasementDoor_C"))
      (Variables|Default|SetA _outactors_7)
      (bind _outactors_8 (Actor|GetAllActorsOfClass "/Game/Leak/Assets/Meshes/Buildings/Basement/Door/BP_BasementDoor_TEST.BP_BasementDoor_TEST_C"))
      (Variables|Default|SetB _outactors_8))))

(fn ConstructionScript)

(fn ChangeInterractDuration
  (params (Duration :type Float%20%28double-precision%29))
  (bind _asbp_interaction_area_custom_shape (Utilities|Casting|CastToBP_InteractionArea_Custom_Shape (Variables|/Script/Engine.ChildActorComponent|GetChildActor (Variables|Default|GetChildActor))))
  (Variables|/Game/Leak/Blueprints/Interaction/InteractionArea/BP_InteractionArea_Master.BP_InteractionArea_Master_C|SetInteractDuration _asbp_interaction_area_custom_shape Duration))