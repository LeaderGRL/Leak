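; AudioTest is a test Blueprint that toggles a bit-crush source effect on the David sound through a Box trigger.
; On begin overlap, it assigns Testchain to David, adds the effect to the chain and raises a preset's sample rate by a fixed, cumulative step.
; On end overlap, it removes the chain's first entry and prints the preset's sample rate value.
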(event OnComponentBeginOverlap(Box)
  (params (OverlappedComponent :type Primitive%20Component%20Object%20Reference) (OtherActor :type Actor%20Object%20Reference) (OtherComp :type Primitive%20Component%20Object%20Reference) (OtherBodyIndex :type Integer) (bFromSweep :type Boolean) (SweepResult :type Hit%20Result%20Structure%20%28by%20ref%29))
  (bind _output_get (Variables|/Script/Engine.AudioComponent|SetSourceEffectChain (Variables|Default|GetDavid) "/Game/Leak/Assets/Audio/testchain.testchain"))
  (Class|AudioMixerBlueprintLibrary|AddSourceEffecttoPresetChain _output_get (Utilities|Struct|MakeSourceEffectChainEntry "/Game/Leak/Assets/Audio/BitCrushEffect.BitCrushEffect" false))
  (bind _output_get_2 (Variables|Default|Setrate (+ (Variables|Default|Getrate) 4e+03)))
  (Class|SourceEffectBitCrusherPreset|SetSampleRate (Variables|Default|Getpreset) _output_get_2))

(event OnComponentEndOverlap(Box)
  (params (OverlappedComponent :type Primitive%20Component%20Object%20Reference) (OtherActor :type Actor%20Object%20Reference) (OtherComp :type Primitive%20Component%20Object%20Reference) (OtherBodyIndex :type Integer))
  (Class|AudioMixerBlueprintLibrary|RemoveSourceEffectfromPresetChain "/Game/Leak/Assets/Audio/testchain.testchain")
  (Development|PrintString (Utilities|String|ToString(Float) (.value (.sampleratemodulation (Variables|/Script/Synthesis.SourceEffectBitCrusherPreset|GetSettings (Variables|Default|Getpreset)))))))

(fn ConstructionScript)