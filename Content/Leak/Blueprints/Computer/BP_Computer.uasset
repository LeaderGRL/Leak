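; Interactable in-world computer that the player takes control of to use its WB_ComputerScreen widget.
; Overlapping InteractBox shows a prompt and enables input; interacting hides the character and weapon, blends the view to the computer and disables character input.
; While controlled, arrow, validate and video-pause inputs drive the screen widget, whose quit event restores the player.
; Quitting starts a shutdown timer that recreates the screen widget unless the player returns first.
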(event OnComponentBeginOverlap(InteractBox)
  (params (OverlappedComponent :type Primitive%20Component%20Object%20Reference) (OtherActor :type Actor%20Object%20Reference) (OtherComp :type Primitive%20Component%20Object%20Reference) (OtherBodyIndex :type Integer) (bFromSweep :type Boolean) (SweepResult :type Hit%20Result%20Structure%20%28by%20ref%29))
  (bind _asbp_first_person_character (Utilities|Casting|CastToBP_FirstPersonCharacter OtherActor))
  (Variables|Default|SetCharaREF _asbp_first_person_character)
  (bind _returnvalue (UserInterface|CreateWidget "/Game/Leak/Blueprints/Interaction/WB_NewInteraction.WB_NewInteraction_C"))
  (UserInterface|Viewport|AddtoViewport _returnvalue 0)
  (Input|EnableInput (Game|GetPlayerController 0)))

(event OnComponentEndOverlap(InteractBox)
  (params (OverlappedComponent :type Primitive%20Component%20Object%20Reference) (OtherActor :type Actor%20Object%20Reference) (OtherComp :type Primitive%20Component%20Object%20Reference) (OtherBodyIndex :type Integer))
  (Utilities|Casting|CastToBP_FirstPersonCharacter OtherActor)
  (bind _foundwidgets (Widget|GetAllWidgetsOfClass "/Game/Leak/Blueprints/Interaction/WB_NewInteraction.WB_NewInteraction_C" true))
  (Widget|RemovefromParent _foundwidgets)
  (Input|DisableInput (Game|GetPlayerController 0)))

(event Custom|Quit
  (bind _asbp_first_person_character (Utilities|Casting|CastToBP_FirstPersonCharacter (Game|GetPlayerCharacter 0)))
  (Default|Hide _asbp_first_person_character)
  (if (not (Variables|/Game/Leak/Blueprints/Character/BP_FirstPersonCharacter.BP_FirstPersonCharacter_C|GetIsHiding _asbp_first_person_character))
    (Default|UnHideWeapon (Variables|Default|GetCharaREF))
    (Utilities|FlowControl|Sequence
      (:then_0
        (if (Variables|Default|GetisControlled)
          (bind _output_get (Variables|Default|SetisControlled false))
          (Utilities|SetPlayerInteractionMode _output_get)
          ;[0 1 0.9297] Create or reset Timer
          (bind _returnvalue (Utilities|Time|SetTimerbyFunctionName 0 "Reset Widget" (* (Variables|Default|GetTime%20Before%20Shutdown%20%28in%20min%29) 6e+01)))
          (Variables|Default|SetTimer _returnvalue)))
      (:then_1
        (Transformation|SetRelativeLocation (Variables|Default|GetInteractBox) "0.000000,97.000000,0.000000" false false)))))

(event Input|EnhancedActionEvents|EnhancedInputActionIA_DirectionalArrow
  (params (ActionValue :type Vector%202D%20Structure) (ElapsedSeconds :type Float%20%28double-precision%29) (TriggeredSeconds :type Float%20%28double-precision%29) (InputAction :type Input%20Action%20Object%20Reference :default "/Game/Leak/Inputs/Actions/IA_DirectionalArrow.IA_DirectionalArrow"))
  (if (Variables|Default|GetisControlled)
    (bind _computer_screen (CallFunction|GetWidget))
    (Default|Select _computer_screen ActionValue)))

(event Input|EnhancedActionEvents|EnhancedInputActionIA_Validate
  (params (ActionValue :type Boolean) (ElapsedSeconds :type Float%20%28double-precision%29) (TriggeredSeconds :type Float%20%28double-precision%29) (InputAction :type Input%20Action%20Object%20Reference :default "/Game/Leak/Inputs/Actions/IA_Validate.IA_Validate"))
  (bind _computer_screen (CallFunction|GetWidget))
  (Default|Validate _computer_screen (Variables|Default|GetPlayer)))

(event Input|EnhancedActionEvents|EnhancedInputActionIA_Interact
  (params (ActionValue :type Boolean) (ElapsedSeconds :type Float%20%28double-precision%29) (TriggeredSeconds :type Float%20%28double-precision%29) (InputAction :type Input%20Action%20Object%20Reference :default "/Game/Leak/Inputs/Actions/IA_Interact.IA_Interact"))
  (bind _timer (Variables|Default|GetTimer))
  (:Started
    (bind _asbp_first_person_character (Utilities|Casting|CastToBP_FirstPersonCharacter (Game|GetPlayerCharacter 0)))
    (Default|Hide _asbp_first_person_character)
    (if (Variables|/Game/Leak/Blueprints/Character/BP_FirstPersonCharacter.BP_FirstPersonCharacter_C|GetIsHiding _asbp_first_person_character)
      (Default|HideWeapon (Variables|Default|GetCharaREF))
      (Transformation|SetRelativeLocation (Variables|Default|GetInteractBox) "0.000000,97.000000,-222.000000" false false)
      (if (not (Variables|Default|GetisControlled))
        (bind _output_get (Variables|Default|SetisControlled true))
        (Utilities|SetPlayerInteractionMode _output_get self)
        (bind _computer_screen (CallFunction|GetWidget))
        (EventDispatchers|BindEventtoQuitEvent _computer_screen (EventDispatchers|CreateEvent :!event Custom|Quit))
        (Default|Starting _computer_screen 0.7 1e+01)
        ;[1 0.1406 0] Reset Timer
        (if (Class|KismetSystemLibrary|TimerExistsHandle _timer)
          (Utilities|Time|ClearandInvalidateTimerbyHandle _timer))))))

(event Input|EnhancedActionEvents|EnhancedInputActionIA_PauseVideo
  (params (ActionValue :type Boolean) (ElapsedSeconds :type Float%20%28double-precision%29) (TriggeredSeconds :type Float%20%28double-precision%29) (InputAction :type Input%20Action%20Object%20Reference :default "/Game/Leak/Inputs/Actions/IA_PauseVideo.IA_PauseVideo"))
  (bind _computer_screen (CallFunction|GetWidget))
  (Default|PauseVideo _computer_screen))

(fn ConstructionScript
  (bind _aswb_computer_screen (Utilities|Casting|CastToWB_ComputerScreen (UserInterface|GetWidget (Variables|Default|GetScreen))))
  (Variables|Default|SetComputer%20Screen _aswb_computer_screen))

(fn ResetWidget
  (if (not (Variables|Default|GetisControlled))
    (bind _computer_screen (CallFunction|GetWidget))
    (Widget|RemovefromParent _computer_screen)
    (CallFunction|SetWidget)
    (bind _returnvalue (UserInterface|CreateWidget "/Game/Leak/Blueprints/Computer/WB_ComputerScreen.WB_ComputerScreen_C"))
    (bind _output_get (Variables|Default|SetComputer%20Screen _returnvalue))
    (CallFunction|SetWidget _output_get)
    (Development|PrintString "Hello")
    (else
      (Utilities|Time|ClearandInvalidateTimerbyHandle (Variables|Default|GetTimer)))))

(fn GetWidget
  (bind _aswb_computer_screen (Utilities|Casting|CastToWB_ComputerScreen (UserInterface|GetWidget (Variables|Default|GetScreen))))
  (return _aswb_computer_screen))

(fn SetWidget
  (params (Widget :type User%20Widget%20Object%20Reference))
  (UserInterface|SetWidget (Variables|Default|GetScreen) Widget))

(fn ToggleHide
  (bind _returnvalue (Game|GetPlayerController 0))
  (bind _chararef (Variables|Default|GetCharaREF))
  (bind _chararef_2 (Variables|Default|GetCharaREF))
  (bind _asbp_first_person_character (Utilities|Casting|CastToBP_FirstPersonCharacter (Game|GetPlayerCharacter 0)))
  (Default|Hide _asbp_first_person_character)
  (if (Variables|/Game/Leak/Blueprints/Character/BP_FirstPersonCharacter.BP_FirstPersonCharacter_C|GetIsHiding _asbp_first_person_character)
    (Rendering|SetActorHiddenInGame _chararef_2 true)
    (Collision|SetActorEnableCollision _chararef_2 false)
    (Game|Player|SetViewTargetwithBlend _returnvalue self 0.8 "VTBlend_Linear" 0.0 false)
    (Transformation|SetActorRelativeLocation _chararef_2 (Transformation|GetWorldLocation (Variables|Default|GetChildActor)))
    (Default|HideWeapon _chararef)
    (else
      (Rendering|SetActorHiddenInGame _chararef_2 false)
      (Collision|SetActorEnableCollision _chararef_2 true)
      (Game|Player|SetViewTargetwithBlend _returnvalue _chararef_2 0.8 "VTBlend_Linear" 0.0 false)
      (Transformation|SetActorRelativeLocation _chararef_2 (Transformation|GetWorldLocation (Variables|Default|GetChildActor)))
      (Default|UnHideWeapon _chararef))))