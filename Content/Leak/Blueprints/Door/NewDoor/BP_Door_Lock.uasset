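; Interactive hinged door barred by a plank, toggled open and closed by the player's interact input.
; The box overlap enables input for BP_FirstPersonCharacter and shows a locked or normal prompt widget, both removed on exit.
; The first interaction knocks the plank off with brief physics, clears the lock and reshapes the trigger, while also toggling the door.
; A reversible Timeline lerps door yaw between closed and open angles, with sounds.
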(event OnComponentBeginOverlap(Box)
  (params (OverlappedComponent :type Primitive%20Component%20Object%20Reference) (OtherActor :type Actor%20Object%20Reference) (OtherComp :type Primitive%20Component%20Object%20Reference) (OtherBodyIndex :type Integer) (bFromSweep :type Boolean) (SweepResult :type Hit%20Result%20Structure%20%28by%20ref%29))
  ;[1 1 1] Open Close Door
  (bind _asbp_first_person_character (Utilities|Casting|CastToBP_FirstPersonCharacter OtherActor))
  (Variables|Default|SetChara%20REF _asbp_first_person_character)
  (if (Variables|Default|GetIsLock?)
    (bind _returnvalue (UserInterface|CreateWidget "/Game/Leak/Blueprints/Interaction/WB_NewInteraction_B.WB_NewInteraction_B_C"))
    (UserInterface|Viewport|AddtoViewport _returnvalue 0)
    (else
      (bind _returnvalue_2 (UserInterface|CreateWidget "/Game/Leak/Blueprints/Interaction/WB_NewInteraction.WB_NewInteraction_C"))
      (UserInterface|Viewport|AddtoViewport _returnvalue_2 0)))
  (Input|EnableInput (Game|GetPlayerController 0))
  (Utilities|FlowControl|Gate true) ; enters at Open
)

(event OnComponentEndOverlap(Box)
  (params (OverlappedComponent :type Primitive%20Component%20Object%20Reference) (OtherActor :type Actor%20Object%20Reference) (OtherComp :type Primitive%20Component%20Object%20Reference) (OtherBodyIndex :type Integer))
  ;[1 1 1] Open Close Door
  (Utilities|Casting|CastToBP_FirstPersonCharacter OtherActor)
  (bind _foundwidgets (Widget|GetAllWidgetsOfClass "/Game/Leak/Blueprints/Interaction/WB_NewInteraction.WB_NewInteraction_C" true))
  (Widget|RemovefromParent _foundwidgets)
  (bind _foundwidgets_2 (Widget|GetAllWidgetsOfClass "/Game/Leak/Blueprints/Interaction/WB_NewInteraction_B.WB_NewInteraction_B_C" true))
  (Widget|RemovefromParent _foundwidgets_2)
  (Input|DisableInput (Game|GetPlayerController 0))
  (Utilities|FlowControl|Gate true) ; enters at Close
)

(event Custom|OpenDoor
  ;[1 1 1] Open Close Door
  (Variables|Default|SetIsOpened? true)
  (Audio|PlaySoundatLocation "/Game/Leak/Assets/Audio/Door/Cue_OpenDoor_02.Cue_OpenDoor_02" (Variables|/Script/Engine.SceneComponent|GetRelativeLocation (Variables|Default|GetSM_LittleGirlDoor_Door)) "0, 0, 0" 1.0 1.0 0.0 0 0 0 0)
  (bind _doortrack (Timeline|Timeline Play)
    (:Update
      (Transformation|SetRelativeRotation (Variables|Default|GetSM_LittleGirlDoor_Door) (Math|Rotator|MakeRotator 0.0 0.0 (Math|Float|Lerp (Variables|Default|GetClose%20Angle) (Variables|Default|GetOpen%20Angle) _doortrack)) false false))))

(event Custom|CloseDoor
  ;[1 1 1] Open Close Door
  (Variables|Default|SetIsOpened? false)
  (Audio|PlaySoundatLocation "/Game/Leak/Assets/Audio/Door/Cue_CloseDoor_01.Cue_CloseDoor_01" (Variables|/Script/Engine.SceneComponent|GetRelativeLocation (Variables|Default|GetSM_LittleGirlDoor_Door)) "0, 0, 0" 1.0 1.0 0.0 0 0 0 0)
  (bind _doortrack (Timeline|Timeline Reverse)
    (:Update
      (Transformation|SetRelativeRotation (Variables|Default|GetSM_LittleGirlDoor_Door) (Math|Rotator|MakeRotator 0.0 0.0 (Math|Float|Lerp (Variables|Default|GetClose%20Angle) (Variables|Default|GetOpen%20Angle) _doortrack)) false false))))

(event Input|EnhancedActionEvents|EnhancedInputActionIA_Interact
  (params (ActionValue :type Boolean) (ElapsedSeconds :type Float%20%28double-precision%29) (TriggeredSeconds :type Float%20%28double-precision%29) (InputAction :type Input%20Action%20Object%20Reference :default "/Game/Leak/Inputs/Actions/IA_Interact.IA_Interact"))
  (bind _sm_plank_b_1 (Variables|Default|GetSM_Plank_B_1))
  ;[1 1 1] Open Close Door
  (:Started
    (Utilities|FlowControl|Sequence
      (:then_0
        (Utilities|FlowControl|DoOnce false
          (:Completed
            (Physics|SetSimulatePhysics _sm_plank_b_1 true)
            (Physics|SetPhysicsLinearVelocity _sm_plank_b_1 "0.000000,-200.000000,0.000000" false "None")
            (Transformation|SetRelativeTransform (Variables|Default|GetBox) (Math|Transform|MakeTransform "0.000000,0.000000,125.000000" "0.000000,90.000000,0.000000" "5.000000,3.000000,4.000000") false false)
            (Variables|Default|SetIsLock? false)
            (Utilities|FlowControl|Delay 2.0)
            (Physics|SetSimulatePhysics (Variables|Default|GetSM_Plank_B_1) false))))
      (:then_1
        (if (Variables|Default|GetIsOpened?)
          (CallFunction|CloseDoor)
          (else
            (CallFunction|OpenDoor)))))))

(fn ConstructionScript)