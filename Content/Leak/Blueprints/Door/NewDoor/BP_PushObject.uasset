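; BP_PushObject is an interactable pallet that the player can knock away once.
; Overlapping its Box with BP_FirstPersonCharacter shows the WB_NewInteraction prompt and enables input on the actor; leaving removes the prompt and disables input.
; IA_Interact turns on physics for the pallet, launches it with a fixed world-space velocity and destroys the trigger Box.
; After a delay, physics simulation switches off again.
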(event OnComponentBeginOverlap(Box)
  (params (OverlappedComponent :type Primitive%20Component%20Object%20Reference) (OtherActor :type Actor%20Object%20Reference) (OtherComp :type Primitive%20Component%20Object%20Reference) (OtherBodyIndex :type Integer) (bFromSweep :type Boolean) (SweepResult :type Hit%20Result%20Structure%20%28by%20ref%29))
  (bind _asbp_first_person_character (Utilities|Casting|CastToBP_FirstPersonCharacter OtherActor))
  (Variables|Default|SetChara%20REF _asbp_first_person_character)
  (bind _returnvalue (UserInterface|CreateWidget "/Game/Leak/Blueprints/Interaction/WB_NewInteraction.WB_NewInteraction_C"))
  (UserInterface|Viewport|AddtoViewport _returnvalue 0)
  (Input|EnableInput (Game|GetPlayerController 0)))

(event OnComponentEndOverlap(Box)
  (params (OverlappedComponent :type Primitive%20Component%20Object%20Reference) (OtherActor :type Actor%20Object%20Reference) (OtherComp :type Primitive%20Component%20Object%20Reference) (OtherBodyIndex :type Integer))
  (Utilities|Casting|CastToBP_FirstPersonCharacter OtherActor)
  (bind _foundwidgets (Widget|GetAllWidgetsOfClass "/Game/Leak/Blueprints/Interaction/WB_NewInteraction.WB_NewInteraction_C" true))
  (Widget|RemovefromParent _foundwidgets)
  (Input|DisableInput (Game|GetPlayerController 0)))

(event Input|EnhancedActionEvents|EnhancedInputActionIA_Interact
  (params (ActionValue :type Boolean) (ElapsedSeconds :type Float%20%28double-precision%29) (TriggeredSeconds :type Float%20%28double-precision%29) (InputAction :type Input%20Action%20Object%20Reference :default "/Game/Leak/Inputs/Actions/IA_Interact.IA_Interact"))
  (bind _sm_pallet_a_1 (Variables|Default|GetSM_Pallet_A_1))
  (:Started
    (Physics|SetSimulatePhysics _sm_pallet_a_1 true)
    (Physics|SetPhysicsLinearVelocity _sm_pallet_a_1 "400.000000,400.000000,0.000000" false "None")
    (Components|DestroyComponent (Variables|Default|GetBox))
    (Utilities|FlowControl|Delay 15.0)
    (Physics|SetSimulatePhysics (Variables|Default|GetSM_Pallet_A_1) false)))

(fn ConstructionScript)