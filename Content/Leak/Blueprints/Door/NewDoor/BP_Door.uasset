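; BP_Door is an interactive door that the first-person character opens and closes with IA_Interact.
; Entering its Box trigger enables input and shows a WB_NewInteraction widget; leaving disables input and removes it.
; Each interaction toggles IsOpened, playing or reversing a Timeline that lerps the mesh yaw between CloseAngle and OpenAngle.
; Open and close sounds play at the mesh's relative location, passed as the world location.
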(event OnComponentBeginOverlap(Box)
  (params (OverlappedComponent :type Primitive%20Component%20Object%20Reference) (OtherActor :type Actor%20Object%20Reference) (OtherComp :type Primitive%20Component%20Object%20Reference) (OtherBodyIndex :type Integer) (bFromSweep :type Boolean) (SweepResult :type Hit%20Result%20Structure%20%28by%20ref%29))
  ;[1 1 1] Open Close Door
  (bind _asbp_first_person_character (Utilities|Casting|CastToBP_FirstPersonCharacter OtherActor))
  (Variables|Default|SetChara%20REF _asbp_first_person_character)
  (bind _returnvalue (UserInterface|CreateWidget "/Game/Leak/Blueprints/Interaction/WB_NewInteraction.WB_NewInteraction_C"))
  (UserInterface|Viewport|AddtoViewport _returnvalue 0)
  (Input|EnableInput (Game|GetPlayerController 0))
  (Utilities|FlowControl|Gate true) ; enters at Open
)

(event OnComponentEndOverlap(Box)
  (params (OverlappedComponent :type Primitive%20Component%20Object%20Reference) (OtherActor :type Actor%20Object%20Reference) (OtherComp :type Primitive%20Component%20Object%20Reference) (OtherBodyIndex :type Integer))
  ;[1 1 1] Open Close Door
  (Utilities|Casting|CastToBP_FirstPersonCharacter OtherActor)
  (bind _foundwidgets (Widget|GetAllWidgetsOfClass "/Game/Leak/Blueprints/Interaction/WB_NewInteraction.WB_NewInteraction_C" true))
  (Widget|RemovefromParent _foundwidgets)
  (Input|DisableInput (Game|GetPlayerController 0))
  (Utilities|FlowControl|Gate true) ; enters at Close
)

(event Custom|OpenDoor
  ;[1 1 1] Open Close Door
  (Variables|Default|SetIsOpened? true)
  (Audio|PlaySoundatLocation "/Game/Leak/Assets/Audio/Door/Cue_OpenDoor_02.Cue_OpenDoor_02" (Variables|/Script/Engine.SceneComponent|GetRelativeLocation (Variables|Default|GetSM_LittleGirlDoor_Door)) "0, 0, 0" 1.0 1.0 0.0 0 0 0 0)
  (bind _doortrack (Timeline|Timeline Play)
    (:Update
      (Transformation|SetRelativeRotation (Variables|Default|GetSM_LittleGirlDoor_Door) (Math|Rotator|MakeRotator 0.0 0.0 (Math|Float|Lerp (Variables|Default|GetClose%20Angle) (Variables|Default|GetOpen%20Angle) _doortrack)) false false))))

(event Custom|CloseDoor
  ;[1 1 1] Open Close Door
  (Variables|Default|SetIsOpened? false)
  (Audio|PlaySoundatLocation "/Game/Leak/Assets/Audio/Door/Cue_CloseDoor_01.Cue_CloseDoor_01" (Variables|/Script/Engine.SceneComponent|GetRelativeLocation (Variables|Default|GetSM_LittleGirlDoor_Door)) "0, 0, 0" 1.0 1.0 0.0 0 0 0 0)
  (bind _doortrack (Timeline|Timeline Reverse)
    (:Update
      (Transformation|SetRelativeRotation (Variables|Default|GetSM_LittleGirlDoor_Door) (Math|Rotator|MakeRotator 0.0 0.0 (Math|Float|Lerp (Variables|Default|GetClose%20Angle) (Variables|Default|GetOpen%20Angle) _doortrack)) false false))))

(event Input|EnhancedActionEvents|EnhancedInputActionIA_Interact
  (params (ActionValue :type Boolean) (ElapsedSeconds :type Float%20%28double-precision%29) (TriggeredSeconds :type Float%20%28double-precision%29) (InputAction :type Input%20Action%20Object%20Reference :default "/Game/Leak/Inputs/Actions/IA_Interact.IA_Interact"))
  ;[1 1 1] Open Close Door
  (:Started
    (if (Variables|Default|GetIsOpened?)
      (CallFunction|CloseDoor)
      (else
        (CallFunction|OpenDoor)))))

(fn ConstructionScript)