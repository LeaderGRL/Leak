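; Interactable hinged door that toggles open and closed by rotating its static mesh in yaw.
; Interface events highlight it through custom depth on focus and trigger Interact, which plays or reverses a timeline lerping between the closed and open angles.
; The construction script applies the configurable mesh and transform, copies the mesh to the child interaction-area shape, and derives timeline play rate from the open/close duration.
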(event Custom|Interact
  (Variables|Default|SetInteractToggle (not (Variables|Default|GetInteractToggle)))
  (if (not (Variables|Default|GetisOpened?))
    (Variables|Default|SetisOpened? true)
    (bind _door_track (Timeline|Timeline Play)
      (:Update
        (Transformation|SetRelativeRotation (Variables|Components|GetStaticMesh) (Math|Rotator|MakeRotator 0.0 0.0 (Math|Float|Lerp (Variables|Default|GetCloseDoor) (Variables|Default|GetDoorAngle) _door_track)) false false)))
    (else
      (Variables|Default|SetisOpened? false)
      (Timeline|Timeline Reverse))))

(event EventInterfaceToggleFocus
  (params (Focus :type Boolean))
  (Rendering|SetRenderCustomDepth (Variables|Components|GetStaticMesh) Focus))

(event EventInterfaceInteract
  (CallFunction|Interact))

(fn ConstructionScript
  (bind _staticmesh (Variables|Components|GetStaticMesh))
  (Utilities|FlowControl|Sequence
    (:then_0
      ;[0 1 0.9062] Set Static Mesh
      (Components|StaticMesh|SetStaticMesh _staticmesh (Variables|Init|GetBasicMesh))
      (Transformation|SetRelativeLocationAndRotation _staticmesh (Variables|Init|GetMesh%20Location) (Variables|Init|GetMesh%20Rotation) false false))
    (:then_1
      ;[0 1 0.9062] Set Child Actor Mesh
      (bind _asbp_interaction_area_custom_shape (Utilities|Casting|CastToBP_InteractionArea_Custom_Shape (Variables|/Script/Engine.ChildActorComponent|GetChildActor (Variables|Components|GetChildActor))))
      (Components|StaticMesh|SetStaticMesh (Variables|/Game/Leak/Blueprints/Interaction/InteractionArea/BP_InteractionArea_Custom_Shape.BP_InteractionArea_Custom_Shape_C|GetShape _asbp_interaction_area_custom_shape) (Variables|Init|GetBasicMesh)))
    (:then_2
      ;[0 1 0.9062] Set Door Speed and Angle
      ;;[1 0.09375 0] Speed
      (Components|Timeline|SetPlayRate (Variables|Default|GetTimeline) (/ 1.0 (Variables|Default|GetOCDuration))))))