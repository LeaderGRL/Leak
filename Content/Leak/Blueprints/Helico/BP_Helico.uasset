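; BP_Helico is an actor, by its name a helicopter, that flies along a referenced spline path once play begins.
; On BeginPlay a timeline plays at a rate of one over TimeToComplete, so that variable controls the travel duration.
; Each update maps the timeline track to a distance along the spline and sets the actor's world location and rotation from that point.
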(event Custom|MoveObject
  (bind _splineref (Variables|Default|GetSplineRef))
  (bind _spline (Variables|/Game/Leak/Blueprints/SplineTool/BP_SplineWireTool.BP_SplineWireTool_C|GetSpline _splineref))
  (Components|Timeline|SetPlayRate (Variables|Default|GetMove%20Object%20T) (/ 1.0 (Variables|Default|GetTimeToComplete)))
  (bind _move_track (Timeline|Move%20Object%20T Play)
    (:Update
      (Transformation|SetActorTransform (Math|Transform|MakeTransform (Spline|GetLocationatDistanceAlongSpline _spline (Math|Float|Lerp 0.0 (Spline|GetSplineLength (Variables|/Game/Leak/Blueprints/SplineTool/BP_SplineWireTool.BP_SplineWireTool_C|GetSpline (Variables|Default|GetSplineRef))) _move_track) "World") (Spline|GetRotationatDistanceAlongSpline _spline (Math|Float|Lerp 0.0 (Spline|GetSplineLength (Variables|/Game/Leak/Blueprints/SplineTool/BP_SplineWireTool.BP_SplineWireTool_C|GetSpline (Variables|Default|GetSplineRef))) _move_track) "World") "1.000000,1.000000,1.000000")))))

(event EventBeginPlay
  (CallFunction|MoveObject))

(fn ConstructionScript)