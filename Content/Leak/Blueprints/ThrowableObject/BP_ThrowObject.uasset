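; Throwable prop that the first-person player can highlight on focus, pick up into the right-hand socket, and throw with the Interact input.
; A timeline scaled by TimeToFly sweeps it along the camera direction while spinning, lowering the target each update to fake an arc.
; A hit or the timeline's end hands the mesh over to physics.
; The construction script applies NewMesh to both the prop and its child interaction-area shape.
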(event Custom|Interact
  (if (not (Variables|/Game/Leak/Blueprints/Character/BP_FirstPersonCharacter.BP_FirstPersonCharacter_C|GetObject%20Attached (Variables|Default|GetChar%20Ref)))
    (Variables|/Game/Leak/Blueprints/Character/BP_FirstPersonCharacter.BP_FirstPersonCharacter_C|SetObject%20Attached (Variables|Default|GetChar%20Ref) true)
    (bind _returnvalue (Transformation|AttachComponentToComponent (Variables|/Game/Leak/Blueprints/Character/BP_FirstPersonCharacter.BP_FirstPersonCharacter_C|GetFirstPersonMesh (Variables|Default|GetChar%20Ref)) "hand_rSocket" "SnapToTarget" "SnapToTarget" "SnapToTarget" true))
    (if _returnvalue
      (Physics|SetSimulatePhysics (Variables|Default|GetStaticMesh) false))))

(event Input|EnhancedActionEvents|EnhancedInputActionIA_Interact
  (params (ActionValue :type Boolean) (ElapsedSeconds :type Float%20%28double-precision%29) (TriggeredSeconds :type Float%20%28double-precision%29) (InputAction :type Input%20Action%20Object%20Reference :default "/Game/Leak/Inputs/Actions/IA_Interact.IA_Interact"))
  (:Started
    (if (Variables|/Game/Leak/Blueprints/Character/BP_FirstPersonCharacter.BP_FirstPersonCharacter_C|GetObject%20Attached (Variables|Default|GetChar%20Ref))
      (Transformation|DetachFromActor "KeepWorld" "KeepWorld" "KeepWorld")
      (Variables|/Game/Leak/Blueprints/Character/BP_FirstPersonCharacter.BP_FirstPersonCharacter_C|SetObject%20Attached (Variables|Default|GetChar%20Ref) false)
      (Collision|SetCollisionEnabled (Variables|Default|GetStaticMesh) "QueryAndPhysics")
      (|Throw))))

(event Collision|EventHit
  (params (MyComp :type Primitive%20Component%20Object%20Reference) (Other :type Actor%20Object%20Reference) (OtherComp :type Primitive%20Component%20Object%20Reference) (bSelfMoved :type Boolean) (HitLocation :type Vector :default "0, 0, 0") (HitNormal :type Vector :default "0, 0, 0") (NormalImpulse :type Vector :default "0, 0, 0") (Hit :type Hit%20Result%20Structure%20%28by%20ref%29))
  (Audio|Components|Audio|Stop (Variables|Default|GetThrowingTL))
  (Physics|SetSimulatePhysics (Variables|Default|GetStaticMesh) true))

(event EventBeginPlay
  (bind _asbp_first_person_character (Utilities|Casting|CastToBP_FirstPersonCharacter (Game|GetPlayerCharacter 0)))
  (Variables|Default|SetChar%20Ref _asbp_first_person_character))

(event EventInterfaceInteract
  (CallFunction|Interact))

(event EventInterfaceToggleFocus
  (params (Focus :type Boolean))
  (Rendering|SetRenderCustomDepth (Variables|Default|GetStaticMesh) Focus))

(fn ConstructionScript
  (Components|Timeline|SetPlayRate (Variables|Default|GetThrowingTL) (/ 1.0 (Variables|Default|GetTime%20to%20fly)))
  (Components|StaticMesh|SetStaticMesh (Variables|Default|GetStaticMesh) (Variables|Default|GetNew%20Mesh))
  (bind _asbp_interaction_area_custom_shape (Utilities|Casting|CastToBP_InteractionArea_Custom_Shape (Variables|/Script/Engine.ChildActorComponent|GetChildActor (Variables|Default|GetChildActor))))
  (Components|StaticMesh|SetStaticMesh (Variables|/Game/Leak/Blueprints/Interaction/InteractionArea/BP_InteractionArea_Custom_Shape.BP_InteractionArea_Custom_Shape_C|GetShape _asbp_interaction_area_custom_shape) (Variables|Default|GetNew%20Mesh)))