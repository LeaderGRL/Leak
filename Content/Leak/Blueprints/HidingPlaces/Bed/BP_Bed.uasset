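; BP_Bed is a hiding place the player can enter and leave with the Interact input.
; Box overlap shows an interaction widget and enables input through a gate.
; ToggleHide hides the character and weapon, disables collision, switches off the point light and blends the view to the bed, reversing this on exit.
; While hiding, look input drives a clamped pitch and yaw, applied to the camera by a self-calling delay loop.
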(event OnComponentBeginOverlap(Box)
  (params (OverlappedComponent :type Primitive%20Component%20Object%20Reference) (OtherActor :type Actor%20Object%20Reference) (OtherComp :type Primitive%20Component%20Object%20Reference) (OtherBodyIndex :type Integer) (bFromSweep :type Boolean) (SweepResult :type Hit%20Result%20Structure%20%28by%20ref%29))
  ;[1 1 1] Get In and Out
  (bind _asbp_first_person_character (Utilities|Casting|CastToBP_FirstPersonCharacter OtherActor))
  (Variables|Default|SetChara%20REF _asbp_first_person_character)
  (bind _returnvalue (UserInterface|CreateWidget "/Game/Leak/Blueprints/Interaction/WB_NewInteraction_C.WB_NewInteraction_C_C"))
  (UserInterface|Viewport|AddtoViewport _returnvalue 0)
  (Input|EnableInput (Game|GetPlayerController 0))
  (Utilities|FlowControl|Gate true) ; enters at Open
)

(event OnComponentEndOverlap(Box)
  (params (OverlappedComponent :type Primitive%20Component%20Object%20Reference) (OtherActor :type Actor%20Object%20Reference) (OtherComp :type Primitive%20Component%20Object%20Reference) (OtherBodyIndex :type Integer))
  (bind _returnvalue (Game|GetPlayerController 0))
  ;[1 1 1] Get In and Out
  (Utilities|Casting|CastToBP_FirstPersonCharacter OtherActor)
  (bind _foundwidgets (Widget|GetAllWidgetsOfClass "/Game/Leak/Blueprints/Interaction/WB_NewInteraction_C.WB_NewInteraction_C_C" true))
  (Widget|RemovefromParent _foundwidgets)
  (Input|DisableInput _returnvalue)
  (Utilities|FlowControl|Gate true) ; enters at Close
)

(event Custom|MoveCamera
  ;[1 1 1] Move Camera
  (if (Variables|Default|GetIsHiding?)
    (Transformation|SetRelativeRotation (Variables|Default|GetCamera) (Math|Rotator|MakeRotator 0.0 (* (stale Input|EnhancedActionEvents|EnhancedInputActionIA_Look _output_get) -1.0) (stale Input|MouseEvents|MouseX _output_get)) false false)
    (Utilities|FlowControl|Delay 0.001)
    (CallFunction|MoveCamera)))

(event Input|EnhancedActionEvents|EnhancedInputActionIA_Interact
  (params (ActionValue :type Boolean) (ElapsedSeconds :type Float%20%28double-precision%29) (TriggeredSeconds :type Float%20%28double-precision%29) (InputAction :type Input%20Action%20Object%20Reference :default "/Game/Leak/Inputs/Actions/IA_Interact.IA_Interact"))
  ;[1 1 1] Get In and Out
  (:Started
    (Utilities|FlowControl|Gate true :!label _label
      (:Exit
        (CallFunction|ToggleHide)
        (CallFunction|MoveCamera)
        (Utilities|FlowControl|Delay 0.2)
        (Input|EnableInput (Game|GetPlayerController 0))
        (goto _label Open)))))

(event Input|EnhancedActionEvents|EnhancedInputActionIA_Look
  (params (ActionValue :type Vector%202D%20Structure) (ElapsedSeconds :type Float%20%28double-precision%29) (TriggeredSeconds :type Float%20%28double-precision%29) (InputAction :type Input%20Action%20Object%20Reference :default "/Game/Leak/Inputs/Actions/IA_Look.IA_Look"))
  ;[1 1 1] Move Camera
  (if (Variables|Default|GetIsHiding?)
    (bind _output_get (Variables|Default|SetPitch (Math|Float|Clamp(Float) (+ (Variables|Default|GetPitch) (.y ActionValue)) -3e+01 2e+01)))))

(event Input|MouseEvents|MouseX
  (params (AxisValue :type Float%20%28single-precision%29))
  ;[1 1 1] Move Camera
  (if (Variables|Default|GetIsHiding?)
    (bind _output_get (Variables|Default|SetYaw (Math|Float|Clamp(Float) (+ (Variables|Default|GetYaw) AxisValue) -4e+01 4e+01)))))

(fn ConstructionScript)

(fn ToggleHide
  (bind _returnvalue (Game|GetPlayerController 0))
  (bind _chara_ref (Variables|Default|GetChara%20REF))
  (if (Variables|Default|GetIsHiding?)
    (Variables|Default|SetIsHiding? false)
    (Rendering|SetActorHiddenInGame _chara_ref false)
    (Collision|SetActorEnableCollision _chara_ref true)
    (Game|Player|SetViewTargetwithBlend _returnvalue _chara_ref 0.8 "VTBlend_Linear" 0.0 false)
    (Rendering|SetVisibility (Variables|Default|GetPointLight) true false)
    (Default|UnHideWeapon (Variables|Default|GetChara%20REF))
    (else
      (Variables|Default|SetIsHiding? true)
      (Rendering|SetActorHiddenInGame _chara_ref true)
      (Collision|SetActorEnableCollision _chara_ref false)
      (Game|Player|SetViewTargetwithBlend _returnvalue self 0.8 "VTBlend_Linear" 0.0 false)
      (Rendering|SetVisibility (Variables|Default|GetPointLight) false false)
      (Default|HideWeapon (Variables|Default|GetChara%20REF)))))