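; Locker hiding spot that moves the first-person player inside and switches to a clamped-look locker camera.
; Interaction flips a RepNotify toggle that swings the door and passes an overlap-controlled gate to Hide or Unhide.
; IA_Hide also exits, and unhiding restores movement and notifies AI_NPC, while the hide-side AI notification is disconnected.
; A recursive Delay loop updates camera rotation; the construction script applies mesh, camera, widget, trigger and interaction-area settings.
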(event OnComponentBeginOverlap(Box)
  (params (OverlappedComponent :type Primitive%20Component%20Object%20Reference) (OtherActor :type Actor%20Object%20Reference) (OtherComp :type Primitive%20Component%20Object%20Reference) (OtherBodyIndex :type Integer) (bFromSweep :type Boolean) (SweepResult :type Hit%20Result%20Structure%20%28by%20ref%29))
  ;[0 1 0.4375] Enable Hiding
  (bind _asbp_first_person_character (Utilities|Casting|CastToBP_FirstPersonCharacter OtherActor))
  (Variables|Hiding|SetCharREF _asbp_first_person_character)
  (Variables|Hiding|SetIsColliding? true)
  (Input|EnableInput (Game|GetPlayerController 0))
  ;[0.1016 1 0] if Hiding is enabled start or stop hiding
  (Utilities|FlowControl|Gate true) ; enters at Open
)

(event OnComponentEndOverlap(Box)
  (params (OverlappedComponent :type Primitive%20Component%20Object%20Reference) (OtherActor :type Actor%20Object%20Reference) (OtherComp :type Primitive%20Component%20Object%20Reference) (OtherBodyIndex :type Integer))
  (bind _returnvalue (Game|GetPlayerController 0))
  ;[0 1 0.4375] Disable Hiding
  (Utilities|Casting|CastToBP_FirstPersonCharacter OtherActor)
  (Variables|Hiding|SetIsColliding? false)
  (Input|DisableInput _returnvalue)
  ;[0.1016 1 0] if Hiding is enabled start or stop hiding
  (Utilities|FlowControl|Gate true) ; enters at Close
)

(event Custom|Unhide
  (bind _charref (Variables|Hiding|GetCharREF))
  (bind _charref_2 (Variables|Hiding|GetCharREF))
  ;[0 1 0.8594] Hide/Unhide
  (Variables|/Game/Leak/Blueprints/Character/BP_FirstPersonCharacter.BP_FirstPersonCharacter_C|SetIsHiding _charref false)
  (Pawn|Components|CharacterMovement|SetMovementMode (Variables|/Script/Engine.Character|GetCharacterMovement _charref) "MOVE_Walking" 0)
  (Game|Player|SetViewTargetwithBlend (Game|GetPlayerController 0) (Variables|Hiding|GetCharREF) 0.5 "VTBlend_Linear" 0.0 false)
  (Utilities|FlowControl|Delay 0.5)
  (Rendering|SetActorHiddenInGame _charref_2 false)
  (Collision|SetCollisionEnabled (Variables|/Script/Engine.Character|GetCapsuleComponent _charref_2) "QueryAndProbe")
  (bind _returnvalue (Actor|GetActorOfClass "/Game/Leak/AI/AI_NPC.AI_NPC_C"))
  (bind _asai_npc (Utilities|Casting|CastToAI_NPC _returnvalue))
  (Default|PlayerUnHiding _asai_npc))

(event Custom|Hide
  (bind _charref (Variables|Hiding|GetCharREF))
  ;[0 1 0.8594] Hide/Unhide
  (Variables|/Game/Leak/Blueprints/Character/BP_FirstPersonCharacter.BP_FirstPersonCharacter_C|SetIsHiding _charref true)
  (Pawn|Components|CharacterMovement|DisableMovement (Variables|/Script/Engine.Character|GetCharacterMovement _charref))
  (Pawn|SetControlRotation (Game|GetPlayerController 0) (Transformation|GetSocketRotation (Variables|Default|GetCamera) "None"))
  (Transformation|SetActorLocation (Game|GetPlayerCharacter 0) (Transformation|GetSocketLocation (Variables|Default|GetStaticMesh) "None") true true)
  (Pawn|Components|CharacterMovement|DisableMovement (Variables|/Script/Engine.Character|GetCharacterMovement (Game|GetPlayerCharacter 0))))

(event Custom|MoveCamera
  ;[1 0.2812 0] Camera Input : Moving and limiting the camera
  (if (Variables|/Game/Leak/Blueprints/Character/BP_FirstPersonCharacter.BP_FirstPersonCharacter_C|GetIsHiding (Variables|Hiding|GetCharREF))
    (Transformation|SetRelativeRotation (Variables|Default|GetCamera) (Math|Rotator|MakeRotator 0.0 (stale Input|EnhancedActionEvents|EnhancedInputActionIA_Look _output_get_2) (stale Input|EnhancedActionEvents|EnhancedInputActionIA_Look _output_get)) false false)
    (Utilities|FlowControl|Delay 0.001)
    (CallFunction|MoveCamera)))

(event Custom|Interract
  ;[0 1 0.4375] Start Hiding
  (Utilities|FlowControl|Sequence
    (:then_0
      (bind _newtrack_0 (Timeline|Timeline Play)
        (:Update
          (Transformation|SetRelativeRotation (Variables|Default|GetSM_Locker_Door) (Math|Rotator|Lerp(Rotator) "0, 0, 0" "0.000000,90.000000,0.000000" _newtrack_0) false false)
          (Utilities|FlowControl|Delay 2.0)
          (Timeline|Timeline Reverse))))
    (:then_1
      (Utilities|FlowControl|Delay 1.0)
      ;[0.1016 1 0] if Hiding is enabled start or stop hiding
      (Utilities|FlowControl|Gate true :!label _label
        (:Exit
          (if (Variables|/Game/Leak/Blueprints/Character/BP_FirstPersonCharacter.BP_FirstPersonCharacter_C|GetIsHiding (Variables|Hiding|GetCharREF))
            (CallFunction|Unhide)
            (else
              (CallFunction|Hide)
              (Utilities|FlowControl|Sequence
                (:then_0
                  (Game|Player|SetViewTargetwithBlend (Game|GetPlayerController 0) self 0.5 "VTBlend_Linear" 0.0 false)
                  (CallFunction|MoveCamera))
                (:then_1
                  (Utilities|FlowControl|Delay 0.2)
                  ;[0 1 0.4375] Enable Hiding
                  (Input|EnableInput (Game|GetPlayerController 0))
                  (goto _label Open))))))))))

(event Custom|InteractOnServer
  ;[0 1 0.2031] Enable Interaction
  (Variables|Default|SetInteractToggle (not (Variables|Default|GetInteractToggle))))

(event Input|EnhancedActionEvents|EnhancedInputActionIA_Hide
  (params (ActionValue :type Boolean) (ElapsedSeconds :type Float%20%28double-precision%29) (TriggeredSeconds :type Float%20%28double-precision%29) (InputAction :type Input%20Action%20Object%20Reference :default "/Game/Leak/Inputs/Actions/IA_Hide.IA_Hide"))
  ;[0 1 0.4375] Stop Hiding
  (if (Variables|/Game/Leak/Blueprints/Character/BP_FirstPersonCharacter.BP_FirstPersonCharacter_C|GetIsHiding (Variables|Hiding|GetCharREF))
    (Utilities|FlowControl|Sequence
      (:then_0
        (bind _newtrack_0 (Timeline|Timeline Play)
          (:Update
            (Transformation|SetRelativeRotation (Variables|Default|GetSM_Locker_Door) (Math|Rotator|Lerp(Rotator) "0, 0, 0" "0.000000,90.000000,0.000000" _newtrack_0) false false)
            (Utilities|FlowControl|Delay 2.0)
            (Timeline|Timeline Reverse))))
      (:then_1
        (Utilities|FlowControl|Delay 1.0)
        (Transformation|SetActorLocation (Game|GetPlayerCharacter 0) (Transformation|GetSocketLocation (Variables|Default|GetTeleport) "None") false true)
        ;[0.1016 1 0] if Hiding is enabled start or stop hiding
        (Utilities|FlowControl|Gate true :!label _label
          (:Exit
            (if (Variables|/Game/Leak/Blueprints/Character/BP_FirstPersonCharacter.BP_FirstPersonCharacter_C|GetIsHiding (Variables|Hiding|GetCharREF))
              (CallFunction|Unhide)
              (else
                (CallFunction|Hide)
                (Utilities|FlowControl|Sequence
                  (:then_0
                    (Game|Player|SetViewTargetwithBlend (Game|GetPlayerController 0) self 0.5 "VTBlend_Linear" 0.0 false)
                    (CallFunction|MoveCamera))
                  (:then_1
                    (Utilities|FlowControl|Delay 0.2)
                    ;[0 1 0.4375] Enable Hiding
                    (Input|EnableInput (Game|GetPlayerController 0))
                    (goto _label Open)))))))))))

(event Input|EnhancedActionEvents|EnhancedInputActionIA_Look
  (params (ActionValue :type Vector%202D%20Structure) (ElapsedSeconds :type Float%20%28double-precision%29) (TriggeredSeconds :type Float%20%28double-precision%29) (InputAction :type Input%20Action%20Object%20Reference :default "/Game/Leak/Inputs/Actions/IA_Look.IA_Look"))
  ;[1 0.2812 0] Camera Input : Moving and limiting the camera
  (if (Variables|/Game/Leak/Blueprints/Character/BP_FirstPersonCharacter.BP_FirstPersonCharacter_C|GetIsHiding (Variables|Hiding|GetCharREF))
    (Utilities|FlowControl|Sequence
      (:then_0
        ;;[0 1 0.7656] Yaw (Z)
        (bind _output_get (Variables|Hiding|SetYaw (Math|Float|Clamp(Float) (+ (* (.x ActionValue) -1.0) (Variables|Hiding|GetYaw)) (Variables|Init|GetMinYaw%20%28Z%29) (Variables|Init|GetMaxYaw%20%28Z%29)))))
      (:then_1
        ;;[0 1 0.7656] Pitch (Y)
        (bind _output_get_2 (Variables|Hiding|SetPitch (Math|Float|Clamp(Float) (+ (* (.y ActionValue) -1.0) (Variables|Hiding|GetPitch)) (Variables|Init|GetMinPitch%20%28Y%29) (Variables|Init|GetMaxPitch%20%28Y%29))))))))

(event EventInterfaceToggleFocus
  (params (Focus :type Boolean))
  ;[0 1 0.2031] Enable Interaction
  (Rendering|SetRenderCustomDepth (Variables|Default|GetStaticMesh) Focus))

(event EventInterfaceInteract
  ;[0 1 0.2031] Enable Interaction
  (CallFunction|InteractonServer))

(fn ConstructionScript
  (bind _camera (Variables|Default|GetCamera))
  (bind _camerarotation (Variables|Init|GetCameraRotation))
  (bind _box (Variables|Default|GetBox))
  (bind (_roll _pitch _yaw) (Math|Rotator|BreakRotator _camerarotation))
  (Utilities|FlowControl|Sequence
    (:then_0
      ;[0 1 0.9063] Set Static Mesh
      (Components|StaticMesh|SetStaticMesh (Variables|Default|GetStaticMesh) (Variables|Init|GetBasicMesh)))
    (:then_1
      ;[0 1 0.9062] Set Camera Parameters
      (Transformation|SetRelativeLocationAndRotation _camera (Variables|Init|GetCameraLocation) _camerarotation false false)
      (Variables|Hiding|SetPitch _pitch)
      (Variables|Hiding|SetYaw _yaw)
      (Camera|SetFieldOfView _camera (Variables|Init|GetCameraFOV)))
    (:then_2
      ;[0 1 0.9062] Set Widget Location
      (Transformation|SetRelativeLocation (Variables|Default|GetWidget) (Variables|Init|GetWidget%20Location) false false))
    (:then_3
      ;[0 1 0.9062] Set Box Collision Parameters
      (Transformation|SetRelativeScale3D _box (Variables|Init|GetBox%20Colision%20Scale))
      (Transformation|SetRelativeLocation _box (Variables|Init|GetBox%20Location) false false))
    (:then_4
      ;[0 1 0.9062] Set Child Actor Mesh
      (bind _asbp_interaction_area_custom_shape (Utilities|Casting|CastToBP_InteractionArea_Custom_Shape (Variables|/Script/Engine.ChildActorComponent|GetChildActor (Variables|Default|GetChildActor))))
      (Variables|/Game/Leak/Blueprints/Interaction/InteractionArea/BP_InteractionArea_Master.BP_InteractionArea_Master_C|SetInteractDuration _asbp_interaction_area_custom_shape (Variables|Init|GetInteract%20Duration))
      (Components|StaticMesh|SetStaticMesh (Variables|/Game/Leak/Blueprints/Interaction/InteractionArea/BP_InteractionArea_Custom_Shape.BP_InteractionArea_Custom_Shape_C|GetShape _asbp_interaction_area_custom_shape) (Variables|Init|GetBasicMesh)))))

(fn OnRepInteractToggle
  (CallFunction|Interract))