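; BP_Basement_Lamp_C is a basement lamp with a mesh, point light and spot light that can be switched on and off.
; TurnOffLight blacks out a mesh material slot and zeroes both lights' intensity.
; Activatelight restores white light at NormalIntensity, setting the lamp material, then immediately replacing it with LightFunctionMaterial.
; BeginPlay assigns that same material as both lights' light function and to the mesh slot.
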(event Custom|Activate%20light
  (bind _pointlight (Variables|Default|GetPointLight))
  (bind _normal_intensity (Variables|Default|GetNormal%20Intensity))
  (Rendering|Material|SetMaterial (Variables|Default|GetSM_Basement_Lamp_1) 1 "/Game/Leak/Assets/Materials/Buildings/Basement/MI_Basement_Lamp_B.MI_Basement_Lamp_B")
  (Rendering|Components|Light|SetLightColor _pointlight "(R=1.000000,G=1.000000,B=1.000000,A=1.000000)" true)
  (Rendering|Components|Light|SetIntensity _pointlight _normal_intensity)
  (Rendering|Components|Light|SetIntensity (Variables|Default|GetSpotLight) _normal_intensity)
  (Rendering|Material|SetMaterial (Variables|Default|GetSM_Basement_Lamp_1) 1 (Variables|Default|GetLight%20Function%20Material)))

(event Custom|Turn%20Off%20Light
  (Rendering|Material|SetMaterial (Variables|Default|GetSM_Basement_Lamp_1) 1 "/Game/Leak/Assets/Materials/Specials/M_Black_Inst1.M_Black_Inst1")
  (Rendering|Components|Light|SetIntensity (Variables|Default|GetPointLight) 0.0))

(event EventBeginPlay
  (bind _light_function_material (Variables|Default|GetLight%20Function%20Material))
  (Rendering|Components|Light|SetLightFunctionMaterial (Variables|Default|GetPointLight) _light_function_material)
  (Rendering|Material|SetMaterial (Variables|Default|GetSM_Basement_Lamp_1) 1 _light_function_material))

(fn ConstructionScript)