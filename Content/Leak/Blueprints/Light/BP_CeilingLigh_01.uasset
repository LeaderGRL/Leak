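; Ceiling lamp actor with a lamp mesh, point light and spot light, configured at BeginPlay from a Variation setting.
; Every variation applies the shared Intensity to both lights.
; The first two variations assign LightFunctionMaterial to the lights, and the second also puts it on a lamp mesh material slot.
; The third clears the light function and gives that slot a glossy plastic material.
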(event EventBeginPlay
  (bind _light_function_material (Variables|Default|GetLight%20Function%20Material))
  (switch int (Variables|Default|GetVariation)
    (:0
      (Rendering|Components|Light|SetIntensity (Variables|Default|GetPointLight) (Variables|Default|GetIntensity))
      (Rendering|Components|Light|SetLightFunctionMaterial (Variables|Default|GetPointLight) (Variables|Default|GetLight%20Function%20Material)))
    (:1
      (Rendering|Components|Light|SetIntensity (Variables|Default|GetPointLight) (Variables|Default|GetIntensity))
      (Rendering|Components|Light|SetLightFunctionMaterial (Variables|Default|GetPointLight) _light_function_material)
      (Rendering|Material|SetMaterial (Variables|Default|GetMesh_Ceiling_Lamp) 1 _light_function_material))
    (:2
      (Rendering|Components|Light|SetIntensity (Variables|Default|GetPointLight) (Variables|Default|GetIntensity))
      (Rendering|Components|Light|SetLightFunctionMaterial (Variables|Default|GetPointLight) 0)
      (Rendering|Material|SetMaterial (Variables|Default|GetMesh_Ceiling_Lamp) 1 "/Game/Victorian_House/Materials/Instance/Tiling/Inst_Plastic_Glossy_02.Inst_Plastic_Glossy_02"))))

(fn ConstructionScript)