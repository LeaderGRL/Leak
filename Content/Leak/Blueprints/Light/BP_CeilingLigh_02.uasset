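; BP_CeilingLigh_02 is a ceiling lamp with a spotlight whose look is selected by a Variation setting.
; At BeginPlay it sets the light intensity, then applies a light function material to the spotlight, to both spotlight and one mesh material slot, or clears it and gives that slot a glossy plastic material.
; The construction script is empty, so these changes appear only at runtime.
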(event EventBeginPlay
  (bind _spotlight (Variables|Default|GetSpotLight))
  (bind _spotlight_2 (Variables|Default|GetSpotLight))
  (bind _light_function_material (Variables|Default|GetLight%20Function%20Material))
  (bind _spotlight_3 (Variables|Default|GetSpotLight))
  (switch int (Variables|Default|GetVariation)
    (:0
      (Rendering|Components|Light|SetIntensity _spotlight_2 (Variables|Default|GetIntensity))
      (Rendering|Components|Light|SetLightFunctionMaterial _spotlight_2 (Variables|Default|GetLight%20Function%20Material)))
    (:1
      (Rendering|Components|Light|SetIntensity _spotlight_3 (Variables|Default|GetIntensity))
      (Rendering|Components|Light|SetLightFunctionMaterial _spotlight_3 _light_function_material)
      (Rendering|Material|SetMaterial (Variables|Default|GetSM_LampCeilingA_06) 1 _light_function_material))
    (:2
      (Rendering|Components|Light|SetIntensity _spotlight (Variables|Default|GetIntensity))
      (Rendering|Components|Light|SetLightFunctionMaterial _spotlight 0)
      (Rendering|Material|SetMaterial (Variables|Default|GetSM_LampCeilingA_06) 1 "/Game/Victorian_House/Materials/Instance/Tiling/Inst_Plastic_Glossy_02.Inst_Plastic_Glossy_02"))))

(fn ConstructionScript)