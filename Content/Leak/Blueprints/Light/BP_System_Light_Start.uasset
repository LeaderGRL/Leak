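; Trigger actor that stages a basement blackout with an explosion, followed by red lighting.
; BeginPlay caches all actors of three basement lamp classes and two door classes.
; The player entering the box (once) or any Interact call switches their lights off, shakes the camera and plays the blast sound.
; After a short delay it activates red light on both door types and lamps A and B, leaving C lamps off.
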(event OnComponentBeginOverlap(Box)
  (params (OverlappedComponent :type Primitive%20Component%20Object%20Reference) (OtherActor :type Actor%20Object%20Reference) (OtherComp :type Primitive%20Component%20Object%20Reference) (OtherBodyIndex :type Integer) (bFromSweep :type Boolean) (SweepResult :type Hit%20Result%20Structure%20%28by%20ref%29))
  (Utilities|Casting|CastToBP_FirstPersonCharacter OtherActor)
  (Utilities|FlowControl|DoOnce false
    (:Completed
      (Utilities|FlowControl|Sequence
        (:then_0
          (for _array_element (Variables|Default|GetLamp%20A)
            (Default|TurnOffLight _array_element)))
        (:then_1
          (for _array_element_2 (Variables|Default|GetLamp%20B)
            (Default|TurnOffLight _array_element_2)))
        (:then_2
          (for _array_element_3 (Variables|Default|GetLamp%20C)
            (Default|TurnOffLight _array_element_3)))
        (:then_3
          (for _array_element_4 (Variables|Default|GetDoor%20A)
            (Default|TurnOffLight _array_element_4)))
        (:then_4
          (for _array_element_5 (Variables|Default|GetDoor%20B)
            (Default|TurnOffLight _array_element_5)))
        (:then_5
          (CameraShakes|StartCameraShake (Game|GetPlayerCameraManager 0) "/Game/Leak/Blueprints/Character/BP_CameraShake.BP_CameraShake_C" 2e+01 "CameraLocal" "0, 0, 0")
          (Audio|PlaySound2D "/Game/Leak/StarterContent/Audio/Explosion02.Explosion02" 1.0 1.0 0.0 0 0)
          (Utilities|FlowControl|Delay 2.5)
          (Utilities|FlowControl|Sequence
            (:then_0
              (for _array_element_6 (Variables|Default|GetLamp%20A)
                (Default|ActiveRedLight _array_element_6)))
            (:then_1
              (for _array_element_7 (Variables|Default|GetLamp%20B)
                (Default|ActiveRedLight _array_element_7)))
            (:then_2
              (for _array_element_8 (Variables|Default|GetDoor%20A)
                (Default|ActiveRedLight _array_element_8)))
            (:then_3
              (for _array_element_9 (Variables|Default|GetDoor%20B)
                (Default|ActiveRedLight _array_element_9)))))))))

(event Custom|Interact
  (Utilities|FlowControl|Sequence
    (:then_0
      (for _array_element (Variables|Default|GetLamp%20A)
        (Default|TurnOffLight _array_element)))
    (:then_1
      (for _array_element_2 (Variables|Default|GetLamp%20B)
        (Default|TurnOffLight _array_element_2)))
    (:then_2
      (for _array_element_3 (Variables|Default|GetLamp%20C)
        (Default|TurnOffLight _array_element_3)))
    (:then_3
      (for _array_element_4 (Variables|Default|GetDoor%20A)
        (Default|TurnOffLight _array_element_4)))
    (:then_4
      (for _array_element_5 (Variables|Default|GetDoor%20B)
        (Default|TurnOffLight _array_element_5)))
    (:then_5
      (CameraShakes|StartCameraShake (Game|GetPlayerCameraManager 0) "/Game/Leak/Blueprints/Character/BP_CameraShake.BP_CameraShake_C" 2e+01 "CameraLocal" "0, 0, 0")
      (Audio|PlaySound2D "/Game/Leak/StarterContent/Audio/Explosion02.Explosion02" 1.0 1.0 0.0 0 0)
      (Utilities|FlowControl|Delay 2.5)
      (Utilities|FlowControl|Sequence
        (:then_0
          (for _array_element_6 (Variables|Default|GetLamp%20A)
            (Default|ActiveRedLight _array_element_6)))
        (:then_1
          (for _array_element_7 (Variables|Default|GetLamp%20B)
            (Default|ActiveRedLight _array_element_7)))
        (:then_2
          (for _array_element_8 (Variables|Default|GetDoor%20A)
            (Default|ActiveRedLight _array_element_8)))
        (:then_3
          (for _array_element_9 (Variables|Default|GetDoor%20B)
            (Default|ActiveRedLight _array_element_9)))))))

(event EventBeginPlay
  (Utilities|FlowControl|Sequence
    (:then_0
      (bind _outactors (Actor|GetAllActorsOfClass "/Game/Leak/Blueprints/Light/BP_Basement_Lamp_A.BP_Basement_Lamp_A_C"))
      (Variables|Default|SetLamp%20A _outactors))
    (:then_1
      (bind _outactors_2 (Actor|GetAllActorsOfClass "/Game/Leak/Blueprints/Light/BP_Basement_Lamp_B.BP_Basement_Lamp_B_C"))
      (Variables|Default|SetLamp%20B _outactors_2))
    (:then_2
      (bind _outactors_3 (Actor|GetAllActorsOfClass "/Game/Leak/Blueprints/Light/BP_Basement_Lamp_C.BP_Basement_Lamp_C_C"))
      (Variables|Default|SetLamp%20C _outactors_3))
    (:then_3
      (bind _outactors_4 (Actor|GetAllActorsOfClass "/Game/Leak/Assets/Meshes/Buildings/Basement/Door/BP_BasementDoor.BP_BasementDoor_C"))
      (Variables|Default|SetDoor%20A _outactors_4))
    (:then_4
      (bind _outactors_5 (Actor|GetAllActorsOfClass "/Game/Leak/Assets/Meshes/Buildings/Basement/Door/BP_BasementDoor_TEST.BP_BasementDoor_TEST_C"))
      (Variables|Default|SetDoor%20B _outactors_5))))

(fn ConstructionScript)