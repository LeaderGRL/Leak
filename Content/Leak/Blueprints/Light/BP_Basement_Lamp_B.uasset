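; BP_Basement_Lamp_B is a basement lamp actor with a mesh and point light that switches between normal, red and off states.
; Three events pair a material swap on the mesh's second slot with a point light update: white or red at configurable intensities, or black at zero.
; BeginPlay assigns one light function material to both the light and that mesh slot, and sets the attenuation radius.
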(event Custom|Activate%20light
  (bind _pointlight (Variables|Default|GetPointLight))
  (Rendering|Material|SetMaterial (Variables|Default|GetSM_Basement_Lamp_1) 1 "/Game/Leak/Assets/Materials/Buildings/Basement/MI_Basement_Lamp_B.MI_Basement_Lamp_B")
  (Rendering|Components|Light|SetLightColor _pointlight "(R=1.000000,G=1.000000,B=1.000000,A=1.000000)" true)
  (Rendering|Components|Light|SetIntensity _pointlight (Variables|Default|GetNormal%20Insensity)))

(event Custom|Active%20Red%20Light
  (bind _pointlight (Variables|Default|GetPointLight))
  (Rendering|Material|SetMaterial (Variables|Default|GetSM_Basement_Lamp_1) 1 "/Game/Leak/Assets/Materials/Buildings/Basement/MI_Basement_Lamp_C.MI_Basement_Lamp_C")
  (Rendering|Components|Light|SetLightColor _pointlight "(R=1.000000,G=0.000000,B=0.000000,A=1.000000)" true)
  (Rendering|Components|Light|SetIntensity _pointlight (Variables|Default|GetRed%20Intensity)))

(event Custom|Turn%20Off%20Light
  (Rendering|Material|SetMaterial (Variables|Default|GetSM_Basement_Lamp_1) 1 "/Game/Leak/Assets/Materials/Specials/M_Black.M_Black")
  (Rendering|Components|Light|SetIntensity (Variables|Default|GetPointLight) 0.0))

(event EventBeginPlay
  (bind _light_function_material (Variables|Default|GetLight%20Function%20Material))
  (Rendering|Components|Light|SetLightFunctionMaterial (Variables|Default|GetPointLight) _light_function_material)
  (Rendering|Material|SetMaterial (Variables|Default|GetSM_Basement_Lamp_1) 1 _light_function_material)
  (Rendering|Lighting|SetAttenuationRadius (Variables|Default|GetPointLight) (Variables|Default|GetAttenuation)))

(fn ConstructionScript)