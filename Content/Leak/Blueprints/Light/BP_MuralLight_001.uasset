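; BP_MuralLight_001 is a wall lamp with a lamp mesh and two point lights, configured by a Variation setting.
; On BeginPlay, both handled variations apply the shared Intensity and light function material to the two lights.
; Variation 1 also puts that light function material on the lamp mesh's second material slot.
; The construction script is empty, so these settings apply only at runtime.
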(event EventBeginPlay
  (bind _light_function_material (Variables|Default|GetLight%20Function%20Material))
  (switch int (Variables|Default|GetVariation)
    (:0
      (Rendering|Components|Light|SetIntensity (Variables|Default|GetPointLight) (Variables|Default|GetIntensity))
      (Rendering|Components|Light|SetLightFunctionMaterial (Variables|Default|GetPointLight) (Variables|Default|GetLight%20Function%20Material)))
    (:1
      (Rendering|Components|Light|SetIntensity (Variables|Default|GetPointLight) (Variables|Default|GetIntensity))
      (Rendering|Components|Light|SetLightFunctionMaterial (Variables|Default|GetPointLight) _light_function_material)
      (Rendering|Material|SetMaterial (Variables|Default|GetMesh_Wall_Lamp_01) 1 _light_function_material))))

(fn ConstructionScript)