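; AI director actor that alternates an NPC between rest and hunt phases around the player.
; Each phase loops on a delay, rolling elapsed time against a probability curve to decide when to switch.
; During rest, the rest curve also gates spawning or despawning the NPC through a spawner.
; While hunting, Tick writes a random reachable point near the player to the Blackboard's LastKnownLocation.
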(event Custom|Rest
  ;[1 1 1] Handle rest, spawning and dispawning
  (CallFunction|SpawnifNeeded)
  (Variables|Default|SetIs%20hunting%20? false)
  (bind _returnvalue (CallFunction|DetermineifChangeState (Variables|Rest|GetRest%20curve) (Variables|Hunt|GetTime%20since%20last%20hunt)))
  (if _returnvalue
    (CallFunction|BeginHunt)
    (else
      (CallFunction|IncrementTimeSinceLastHunt)
      (Utilities|FlowControl|Delay (Variables|Default|GetCheck%20every%20sec))
      (CallFunction|Rest))))

(event Custom|Hunt
  ;[1 1 1] Handle hunt
  (Variables|Default|SetIs%20hunting%20? true)
  (bind _returnvalue (CallFunction|DetermineifChangeState (Variables|Hunt|GetHunt%20curve) (Variables|Rest|GetTime%20since%20last%20rest)))
  (if _returnvalue
    (CallFunction|BeginRest)
    (else
      (CallFunction|IncrementTimeSinceLastRest)
      (Utilities|FlowControl|Delay (Variables|Default|GetCheck%20every%20sec))
      (CallFunction|Hunt))))

(event EventTick
  (params (DeltaSeconds :type Float%20%28single-precision%29))
  (bind _blackboard (Variables|NPC|GetBlackboard))
  (if (Variables|Default|GetIs%20hunting%20?)
    (Utilities|IsValid _blackboard
      (:Is%20Valid
        (AI|Components|Blackboard|SetValueasVector _blackboard (Utilities|Name|MakeLiteralName "LastKnownLocation") (.RandomLocation (AI|Navigation|GetRandomReachablePointinRadius (Transformation|GetWorldLocation (Variables|/Script/Engine.Character|GetMesh (Variables|Default|GetPlayer))) (Variables|Default|GetSearchRadius) 0 0)))))))

(event EventBeginPlay
  (bind _returnvalue (Actor|GetActorOfClass "/Game/Leak/Blueprints/Character/BP_FirstPersonCharacter.BP_FirstPersonCharacter_C"))
  (Variables|Default|SetPlayer _returnvalue)
  (CallFunction|Rest))

(fn ConstructionScript)

(fn BeginHunt
  (Utilities|IsValid (Variables|NPC|GetNpc)
    (:Is%20Valid
      (Variables|Hunt|SetTime%20since%20last%20hunt 0.0)
      (CallFunction|Hunt))))

(fn BeginRest
  (Variables|Rest|SetTime%20since%20last%20rest 0.0)
  (CallFunction|Rest))

(fn IncrementTimeSinceLastHunt
  (Variables|Hunt|SetTime%20since%20last%20hunt (+ (Variables|Hunt|GetTime%20since%20last%20hunt) (Variables|Default|GetCheck%20every%20sec))))

(fn IncrementTimeSinceLastRest
  (Variables|Rest|SetTime%20since%20last%20rest (+ (Variables|Rest|GetTime%20since%20last%20rest) (Variables|Default|GetCheck%20every%20sec))))

(fn DetermineifChangeState
  (params (Curve :type Curve%20Float%20Object%20Reference) (Time%20since%20 :type Float%20%28double-precision%29))
  (return (>= (Math|Curves|GetFloatValue Curve Time%20since%20) (Math|Random|RandomFloatinRange 0.0 1e+02))))

(fn SpawnifNeeded
  (bind _spawner (Variables|Default|GetSpawner))
  ;[1 1 1] Dispawn NPC during the beginning of the rest and after amount of time spawn npc.
  (if (> (Math|Curves|GetFloatValue (Variables|Rest|GetRest%20curve) (Variables|Hunt|GetTime%20since%20last%20hunt)) 0.5)
    (bind _output_get (Default|Spawn _spawner))
    (Utilities|IsValid _output_get
      (:Is%20Valid
        (bind _output_get_2 (Variables|NPC|SetNpc _output_get))
        (Variables|NPC|SetBlackboard (AI|GetBlackboard _output_get_2))))
    (else
      (Default|Dispawn _spawner (Variables|NPC|GetBlackboard))
      (Variables|NPC|SetBlackboard 0))))