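; BP_Spawner is an AI utility Blueprint that spawns and despawns a single NPC of a given class.
; SpawnNpc creates an NpcClass actor at the spawner's location and rotation and stores it in Npc, but only when no valid NPC already exists.
; DispawnNpc destroys the stored NPC and clears the reference.
; Neither function is triggered within the Blueprint itself.
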(fn ConstructionScript)

(fn SpawnNpc
  (bind _returnvalue (Transformation|GetActorTransform))
  (Utilities|IsValid (Variables|Default|GetNpc)
    (:Is%20Not%20Valid
      (bind _returnvalue_2 (Game|SpawnActorfromClass (Variables|Default|GetNpc%20class) (Math|Transform|MakeTransform (.location _returnvalue) (.rotation _returnvalue) "1.000000,1.000000,1.000000") "Undefined" "MultiplyWithRoot" 0 0))
      (bind _output_get (Variables|Default|SetNpc _returnvalue_2))
      (return _output_get))))

(fn DispawnNpc
  (Utilities|IsValid (Variables|Default|GetNpc)
    (:Is%20Valid
      (Actor|DestroyActor (Variables|Default|GetNpc))
      (Variables|Default|SetNpc 0))))