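; BP_SpawnerManager keeps an NPC present in the level and assigns it a random spawner as a despawn destination.
; A one-second loop from BeginPlay calls Spawn, which creates a BP_NPC running BT_NPC at a random spawner only when none exists.
; Dispawn writes a random spawner location to the supplied Blackboard once, guarded by IsDispawning, whose reset is unconnected.
; Timer-based and per-spawner spawn loops are also left unconnected.
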(event Custom|SpawnMonster
  (CallFunction|Spawn)
  (Development|PrintString "Hello"))

(event EventBeginPlay
  (for _index (range 0 0) :!label _label
    (CallFunction|Spawn))
  (Utilities|FlowControl|Delay 1.0)
  (goto _label))

(event EventTick
  (params (DeltaSeconds :type Float%20%28single-precision%29)))

(fn ConstructionScript)

(fn Spawn
  (bind _outactors (Actor|GetAllActorsOfClass "/Game/Leak/AI/BP_NPC.BP_NPC_C"))
  (Utilities|IsValid (Utilities|Array|Get(acopy) _outactors)
    (:Is%20Not%20Valid
      (bind _result (Math|Integer|DecrementInt (Utilities|Array|Length (Variables|Default|GetSpawners)))
        (:%20%20
          (bind _returnvalue (AI|SpawnAIFromClass "/Game/Leak/AI/BP_NPC.BP_NPC_C" "/Game/Leak/AI/BT_NPC.BT_NPC" (.location (Transformation|GetActorTransform (Utilities|Array|Get(acopy) (Variables|Default|GetSpawners) (Math|Random|RandomIntegerinRange 0 _result)))) (.rotation (Transformation|GetActorTransform (Utilities|Array|Get(acopy) (Variables|Default|GetSpawners) (Math|Random|RandomIntegerinRange 0 _result)))) false 0))
          (bind _asbp_npc (Utilities|Casting|CastToBP_NPC _returnvalue))
          (return _asbp_npc))))))

(fn Dispawn
  (params (Blackboard :type Blackboard%20Component%20Object%20Reference))
  (if (not (Variables|Default|GetIsDispawning))
    (Utilities|IsValid Blackboard
      (:Is%20Valid
        (bind _result (Math|Integer|DecrementInt (Utilities|Array|Length (Variables|Default|GetSpawners)))
          (:%20%20
            (AI|Components|Blackboard|SetValueasVector Blackboard (Utilities|Name|MakeLiteralName "DispawnLocation") (.location (Transformation|GetActorTransform (Utilities|Array|Get(acopy) (Variables|Default|GetSpawners) (Math|Random|RandomIntegerinRange 0 _result)))))
            (Variables|Default|SetIsDispawning true)))))))