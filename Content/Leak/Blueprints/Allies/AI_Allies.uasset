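; AI controller for allied BP_Allies characters that runs BT_Allies and moves its pawn along the ally's assigned spline.
; Setup sends the ally to the spline's location and scales a timeline's play rate from spline length and max walk speed.
; The timeline issues MoveToLocation toward successive spline points.
; Start, stop and restart events track whether the player is behind, and control playback only when not patrolling.
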(event Custom|Stop%20Run
  (Variables|Default|SetIsPlayerBehind false)
  (if (not (Variables|Default|GetIsPatrolling))
    (bind _alpha (Timeline|Timeline Stop)
      (:Update
        (Variables|Default|SetAlpha _alpha)
        (AI|Navigation|MovetoLocation (Spline|GetLocationatDistanceAlongSpline (Variables|/Game/Leak/Blueprints/Allies/BP_Spline_Allies.BP_Spline_Allies_C|GetSpline (Variables|Default|GetSpline)) (Math|Float|Lerp 0.0 (Spline|GetSplineLength (Variables|/Game/Leak/Blueprints/Allies/BP_Spline_Allies.BP_Spline_Allies_C|GetSpline (Variables|Default|GetSpline))) (Variables|Default|GetAlpha)) "World") 5.0 true true false true 0)))))

(event Custom|Start%20run
  (Variables|Default|SetIsPlayerBehind true)
  (if (not (Variables|Default|GetIsPatrolling))
    (bind _alpha (Timeline|Timeline Play)
      (:Update
        (Variables|Default|SetAlpha _alpha)
        (AI|Navigation|MovetoLocation (Spline|GetLocationatDistanceAlongSpline (Variables|/Game/Leak/Blueprints/Allies/BP_Spline_Allies.BP_Spline_Allies_C|GetSpline (Variables|Default|GetSpline)) (Math|Float|Lerp 0.0 (Spline|GetSplineLength (Variables|/Game/Leak/Blueprints/Allies/BP_Spline_Allies.BP_Spline_Allies_C|GetSpline (Variables|Default|GetSpline))) (Variables|Default|GetAlpha)) "World") 5.0 true true false true 0)))))

(event Custom|Restart%20run
  (CallFunction|PrepareRun (Variables|Default|GetAllies))
  (if (Variables|Default|GetIsPlayerBehind)
    (if (not (Variables|Default|GetIsPatrolling))
      (bind _alpha (Timeline|Timeline PlayFromStart)
        (:Update
          (Variables|Default|SetAlpha _alpha)
          (AI|Navigation|MovetoLocation (Spline|GetLocationatDistanceAlongSpline (Variables|/Game/Leak/Blueprints/Allies/BP_Spline_Allies.BP_Spline_Allies_C|GetSpline (Variables|Default|GetSpline)) (Math|Float|Lerp 0.0 (Spline|GetSplineLength (Variables|/Game/Leak/Blueprints/Allies/BP_Spline_Allies.BP_Spline_Allies_C|GetSpline (Variables|Default|GetSpline))) (Variables|Default|GetAlpha)) "World") 5.0 true true false true 0))))))

(event EventBeginPlay
  (AI|RunBehaviorTree "/Game/Leak/Blueprints/Allies/BT_Allies.BT_Allies")
  (bind _asbp_allies (Utilities|Casting|CastToBP_Allies (Pawn|GetControlledPawn)))
  (bind _output_get (Variables|Default|SetAllies _asbp_allies))
  (CallFunction|PrepareRun _output_get))

(fn ConstructionScript
  (|CallParentFunction))

(fn CalculateDuration
  (Variables|Default|SetDuration (/ (Spline|GetSplineLength (Variables|/Game/Leak/Blueprints/Allies/BP_Spline_Allies.BP_Spline_Allies_C|GetSpline (Variables|Default|GetSpline))) (Variables|/Script/Engine.CharacterMovementComponent|GetMaxWalkSpeed (Variables|/Script/Engine.Character|GetCharacterMovement (Variables|Default|GetAllies))))))

(fn PrepareRun
  (params (Allies :type BP%20Allies%20Object%20Reference))
  (bind _bp_spline (Variables|/Game/Leak/Blueprints/Allies/BP_Allies.BP_Allies_C|GetBP_Spline Allies))
  (Variables|Default|SetSpline _bp_spline)
  (CallFunction|CalculateDuration)
  (Components|Timeline|SetPlayRate (Variables|Default|GetTimeline) (/ 1.0 (Variables|Default|GetDuration)))
  (AI|Navigation|MovetoLocation (Transformation|GetWorldLocation (Variables|/Game/Leak/Blueprints/Allies/BP_Spline_Allies.BP_Spline_Allies_C|GetSpline _bp_spline)) 2.0 true true false true 0))