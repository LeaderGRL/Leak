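; BP_Allies is an allied AI pawn that reacts to the player's proximity.
; On BeginPlay it caches its AI_Allies controller.
; When BP_FirstPersonCharacter begins overlapping its Capsule component, it calls StartRun on that controller and sets IsMoving; when the overlap ends, it calls StopRun and clears the flag.
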(event OnComponentBeginOverlap(Capsule)
  (params (OverlappedComponent :type Primitive%20Component%20Object%20Reference) (OtherActor :type Actor%20Object%20Reference) (OtherComp :type Primitive%20Component%20Object%20Reference) (OtherBodyIndex :type Integer) (bFromSweep :type Boolean) (SweepResult :type Hit%20Result%20Structure%20%28by%20ref%29))
  (Utilities|Casting|CastToBP_FirstPersonCharacter OtherActor)
  (Default|StartRun (Variables|Default|GetAs%20AI%20Allies))
  (Variables|Default|SetIsMoving true))

(event OnComponentEndOverlap(Capsule)
  (params (OverlappedComponent :type Primitive%20Component%20Object%20Reference) (OtherActor :type Actor%20Object%20Reference) (OtherComp :type Primitive%20Component%20Object%20Reference) (OtherBodyIndex :type Integer))
  (Utilities|Casting|CastToBP_FirstPersonCharacter OtherActor)
  (Default|StopRun (Variables|Default|GetAs%20AI%20Allies))
  (Variables|Default|SetIsMoving false))

(event EventBeginPlay
  (bind _asai_allies (Utilities|Casting|CastToAI_Allies (AI|GetAIController self)))
  (Variables|Default|SetAs%20AI%20Allies _asai_allies))

(fn ConstructionScript)