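; BP_Trigger_SearchZone is a box trigger that starts or ends area searching for all BP_Allies when the first-person character crosses it.
; An IsEnterSearchZone flag selects its role: start on overlap begin, or end on overlap end.
; Starting writes search radius and center to each ally's blackboard and enables patrolling on AI_Allies.
; Ending zeroes those keys, assigns the next spline, disables patrolling and restarts the run.
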(event OnComponentBeginOverlap(Box)
  (params (OverlappedComponent :type Primitive%20Component%20Object%20Reference) (OtherActor :type Actor%20Object%20Reference) (OtherComp :type Primitive%20Component%20Object%20Reference) (OtherBodyIndex :type Integer) (bFromSweep :type Boolean) (SweepResult :type Hit%20Result%20Structure%20%28by%20ref%29))
  (if (Variables|Default|GetIsEnterSearchZone)
    (Utilities|Casting|CastToBP_FirstPersonCharacter OtherActor)
    (for _array_element (Variables|Default|GetAllies)
      (AI|Components|Blackboard|SetValueasFloat (AI|GetBlackboard _array_element) (Variables|Default|GetKeySearchRadius) (Variables|Default|GetSearchRadius))
      (AI|Components|Blackboard|SetValueasVector (AI|GetBlackboard _array_element) (Variables|Default|GetKeyPointToSearch) (Transformation|GetWorldLocation (Variables|Default|GetSearchCenter)))
      (bind _asai_allies (Utilities|Casting|CastToAI_Allies (AI|GetAIController _array_element)))
      (Variables|/Game/Leak/Blueprints/Allies/AI_Allies.AI_Allies_C|SetIsPatrolling _asai_allies true))))

(event OnComponentEndOverlap(Box)
  (params (OverlappedComponent :type Primitive%20Component%20Object%20Reference) (OtherActor :type Actor%20Object%20Reference) (OtherComp :type Primitive%20Component%20Object%20Reference) (OtherBodyIndex :type Integer))
  (if (not (Variables|Default|GetIsEnterSearchZone))
    (Utilities|Casting|CastToBP_FirstPersonCharacter OtherActor)
    (for _array_element (Variables|Default|GetAllies)
      (AI|Components|Blackboard|SetValueasFloat (AI|GetBlackboard _array_element) (Variables|Default|GetKeySearchRadius) 0.0)
      (AI|Components|Blackboard|SetValueasVector (AI|GetBlackboard _array_element) (Variables|Default|GetKeyPointToSearch) "0, 0, 0")
      (Variables|/Game/Leak/Blueprints/Allies/BP_Allies.BP_Allies_C|SetBP_Spline _array_element (Variables|Default|GetNextSpline))
      (bind _asai_allies (Utilities|Casting|CastToAI_Allies (AI|GetAIController _array_element)))
      (Variables|/Game/Leak/Blueprints/Allies/AI_Allies.AI_Allies_C|SetIsPatrolling _asai_allies false)
      (Default|RestartRun _asai_allies))))

(event EventBeginPlay
  (bind _outactors (Actor|GetAllActorsOfClass "/Game/Leak/Blueprints/Allies/BP_Allies.BP_Allies_C"))
  (Variables|Default|SetAllies _outactors))

(fn ConstructionScript)