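; BP_NarrowPassage is a trigger actor that scripts the first-person character's entry into and exit from a narrow passage.
; Overlapping StartBox calls StartNarrow once, repositions Box and plays a timeline that slides the character between start markers while turning the view.
; Leaving EndBox calls EndNarrow, then a second timeline moves the character between end markers, turns the view back and rotates Cube.
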(event OnComponentBeginOverlap(StartBox)
  (params (OverlappedComponent :type Primitive%20Component%20Object%20Reference) (OtherActor :type Actor%20Object%20Reference) (OtherComp :type Primitive%20Component%20Object%20Reference) (OtherBodyIndex :type Integer) (bFromSweep :type Boolean) (SweepResult :type Hit%20Result%20Structure%20%28by%20ref%29))
  (bind _chara_ref (Variables|Default|GetChara%20REF))
  (Utilities|FlowControl|DoOnce false
    (:Completed
      (Default|StartNarrow (Variables|Default|GetChara%20REF))
      (Transformation|SetRelativeLocation (Variables|Default|GetBox) "0.000000,21.000000,100.000000" false false)
      (bind _newtrack_0 (Timeline|MovePlayer Play)
        (:Update
          (Transformation|SetActorLocation _chara_ref (Math|Vector|Lerp(Vector) (Transformation|GetWorldLocation (Variables|Default|GetStart1)) (Transformation|GetWorldLocation (Variables|Default|GetStart2)) _newtrack_0) false false)
          (Default|LookLeftRight _chara_ref 0.15))))))

(event OnComponentEndOverlap(EndBox)
  (params (OverlappedComponent :type Primitive%20Component%20Object%20Reference) (OtherActor :type Actor%20Object%20Reference) (OtherComp :type Primitive%20Component%20Object%20Reference) (OtherBodyIndex :type Integer))
  (bind _chara_ref (Variables|Default|GetChara%20REF))
  (Default|EndNarrow (Variables|Default|GetChara%20REF))
  (bind _newtrack_0 (Timeline|Timeline Play)
    (:Update
      (Transformation|SetActorLocation _chara_ref (Math|Vector|Lerp(Vector) (Transformation|GetWorldLocation (Variables|Default|GetEnd1)) (Transformation|GetWorldLocation (Variables|Default|GetEnd2)) _newtrack_0) false false)
      (Default|LookLeftRight _chara_ref -0.15)
      (Transformation|SetRelativeRotation (Variables|Default|GetCube) "40.000000,0.000000,0.000000" false false))))

(event EventBeginPlay
  (Utilities|FlowControl|DoOnce false
    (:Completed
      (bind _returnvalue (Actor|GetActorOfClass "/Game/Leak/Blueprints/Character/BP_FirstPersonCharacter.BP_FirstPersonCharacter_C"))
      (Variables|Default|SetChara%20REF _returnvalue))))

(fn ConstructionScript)