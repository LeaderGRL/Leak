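; Ammo pickup actor that shows its amount on a widget and toggles custom depth rendering on its mesh when focused.
; Interacting adds its amount to the first slot of the player's inventory, capped at that slot's maximum.
; If the total fits, the pickup destroys itself; otherwise it keeps the remainder and refreshes its widget.
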(event Custom|Interact
  (Variables|Default|SetInteractToggle (not (Variables|Default|GetInteractToggle)))
  (CallFunction|AddAmmo self))

(event EventBeginPlay
  (CallFunction|ChangeWidgetValue))

(event EventInterfaceInteract
  (CallFunction|Interact))

(event EventInterfaceToggleFocus
  (params (Focus :type Boolean))
  (Rendering|SetRenderCustomDepth (Variables|Default|GetAmmo) Focus))

(fn ConstructionScript
  (|CallParentFunction))

(fn AddAmmo
  (params (Ref%20Item :type BP%20Main%20Item%20Inventory%20Object%20Reference))
  (bind _inventory (Utilities|GetInventory))
  (bind _s_iteminventory (Variables|/Game/Leak/Blueprints/Inventory/BP_MainItemInventory.BP_MainItemInventory_C|Gets_ItemInventory Ref%20Item))
  (bind (_lessthanmax _amount _remainder) (Utilities|Results _inventory (.amount _s_iteminventory) (.maxamount _s_iteminventory)))
  (Variables|Default|SetAmmoAmount _amount)
  (if _lessthanmax
    (Utilities|FlowControl|Sequence
      (:then_0
        (CallFunction|ChangeInventory (Utilities|GetInventory) (Variables|Default|GetAmmoAmount) :!label _label))
      (:then_1
        (Actor|DestroyActor)))
    (else
      (CallFunction|ChangeAmountItem Ref%20Item _remainder)
      (CallFunction|ChangeWidgetValue)
      (goto _label))))

(fn ChangeWidgetValue
  (bind _aswidget_ammo (Utilities|Casting|CastToWidget_Ammo (UserInterface|GetWidget (Variables|Default|GetAmmoNbr))))
  (Default|ChangeAmmo _aswidget_ammo (.amount (Variables|Default|Gets_ItemInventory))))

(fn ChangeAmountItem
  (params (Item%20Data :type BP%20Main%20Item%20Inventory%20Object%20Reference) (Amount :type Integer))
  (Variables|/Game/Leak/Blueprints/Inventory/BP_MainItemInventory.BP_MainItemInventory_C|Sets_ItemInventory Item%20Data (Utilities|Struct|MakeS_ItemsInventory (.name (Variables|Default|Gets_ItemInventory)) (.description (Variables|Default|Gets_ItemInventory)) (.type (Variables|Default|Gets_ItemInventory)) Amount (.maxamount (Variables|Default|Gets_ItemInventory)))))

(fn ChangeInventory
  (params (Inventory :type Array%20of%20S%20Items%20Inventory%20Structures) (Amount :type Integer))
  (bind _output (Utilities|Array|Get(acopy) Inventory))
  (Utilities|Array|SetArrayElem Inventory 0 (Utilities|Struct|MakeS_ItemsInventory (.name _output) (.description _output) (.type _output) Amount (.maxamount _output))))