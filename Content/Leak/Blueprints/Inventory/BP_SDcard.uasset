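; BP_SDcard is an SD card pickup that the player collects into the first-person character's inventory.
; Overlapping its box outlines the mesh, shows an interaction prompt widget and enables input on the actor, all reversed when overlap ends.
; The Interact input appends the card's item data to the character's Inventory, then hides the actor and disables its collision rather than destroying it.
; A second widget appears briefly after pickup.
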(event OnComponentBeginOverlap(Box)
  (params (OverlappedComponent :type Primitive%20Component%20Object%20Reference) (OtherActor :type Actor%20Object%20Reference) (OtherComp :type Primitive%20Component%20Object%20Reference) (OtherBodyIndex :type Integer) (bFromSweep :type Boolean) (SweepResult :type Hit%20Result%20Structure%20%28by%20ref%29))
  (bind _asbp_first_person_character (Utilities|Casting|CastToBP_FirstPersonCharacter OtherActor))
  (Variables|Default|SetChara%20REF _asbp_first_person_character)
  (Rendering|Material|SetOverlayMaterial (Variables|Default|GetSD) "/Game/Leak/Blueprints/HidingPlaces/MI_Outline.MI_Outline" :!class /Script/Engine.MeshComponent)
  (bind _returnvalue (UserInterface|CreateWidget "/Game/Leak/Blueprints/Interaction/WB_NewInteraction_D.WB_NewInteraction_D_C"))
  (UserInterface|Viewport|AddtoViewport _returnvalue 0)
  (Input|EnableInput (Game|GetPlayerController 0)))

(event OnComponentEndOverlap(Box)
  (params (OverlappedComponent :type Primitive%20Component%20Object%20Reference) (OtherActor :type Actor%20Object%20Reference) (OtherComp :type Primitive%20Component%20Object%20Reference) (OtherBodyIndex :type Integer))
  (Utilities|Casting|CastToBP_FirstPersonCharacter OtherActor)
  (Rendering|Material|SetOverlayMaterial (Variables|Default|GetSD) 0 :!class /Script/Engine.MeshComponent)
  (bind _foundwidgets (Widget|GetAllWidgetsOfClass "/Game/Leak/Blueprints/Interaction/WB_NewInteraction_D.WB_NewInteraction_D_C" true))
  (Widget|RemovefromParent _foundwidgets)
  (Input|DisableInput (Game|GetPlayerController 0)))

(event Input|EnhancedActionEvents|EnhancedInputActionIA_Interact
  (params (ActionValue :type Boolean) (ElapsedSeconds :type Float%20%28double-precision%29) (TriggeredSeconds :type Float%20%28double-precision%29) (InputAction :type Input%20Action%20Object%20Reference :default "/Game/Leak/Inputs/Actions/IA_Interact.IA_Interact"))
  (CallFunction|AddItem self)
  (bind _returnvalue (UserInterface|CreateWidget "/Game/Leak/Blueprints/Interaction/WB_NewInteraction_F.WB_NewInteraction_F_C"))
  (UserInterface|Viewport|AddtoViewport _returnvalue 0)
  (Utilities|FlowControl|Delay 2.0)
  (bind _foundwidgets (Widget|GetAllWidgetsOfClass "/Game/Leak/Blueprints/Interaction/WB_NewInteraction_F.WB_NewInteraction_F_C" true))
  (Widget|RemovefromParent _foundwidgets))

(fn ConstructionScript
  (|CallParentFunction))

(fn AddItem
  (params (Item%20Ref :type BP%20Main%20Item%20Inventory%20Object%20Reference))
  (bind _asbp_first_person_character (Utilities|Casting|CastToBP_FirstPersonCharacter (Game|GetPlayerCharacter 0)))
  (Utilities|Array|Add (Variables|/Game/Leak/Blueprints/Character/BP_FirstPersonCharacter.BP_FirstPersonCharacter_C|GetInventory _asbp_first_person_character) (Variables|/Game/Leak/Blueprints/Inventory/BP_MainItemInventory.BP_MainItemInventory_C|Gets_ItemInventory Item%20Ref))
  (Rendering|SetActorHiddenInGame true)
  (Collision|SetActorEnableCollision false))