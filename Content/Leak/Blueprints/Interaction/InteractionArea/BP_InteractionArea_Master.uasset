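; Base interaction area actor that works on behalf of its parent actor, handling focus and eligibility for player interaction.
; On BeginPlay it finds the parent's shape component tagged "box" and widget component tagged "interact".
; Toggling focus notifies the parent through an interface message and shows or hides the widget.
; Box overlaps reset the overlapping actor's interaction trace, and CanFocus can optionally require the character inside the box.
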(event Custom|ToggleFocus
  (params (Focused :type Boolean))
  (Variables|Default|SetFocused Focused)
  (Class|BIInteraction|InterfaceToggleFocus(Message) (Actor|GetParentActor) (Variables|Default|GetFocused))
  (Development|SetHiddeninGame (Variables|Default|GetInteractWidgetCompRef) (not (Variables|Default|GetFocused)) false))

(event Custom|OnComponentBeginOverlap_Event
  (params (OverlappedComponent :type Primitive%20Component%20Object%20Reference) (OtherActor :type Actor%20Object%20Reference) (OtherComp :type Primitive%20Component%20Object%20Reference) (OtherBodyIndex :type Integer) (bFromSweep :type Boolean) (SweepResult :type Hit%20Result%20Structure%20%28by%20ref%29))
  (Class|BIInteraction|ResetInteractionTrace(Message) OtherActor))

(event Custom|OnComponentEndOverlap_Event
  (params (OverlappedComponent :type Primitive%20Component%20Object%20Reference) (OtherActor :type Actor%20Object%20Reference) (OtherComp :type Primitive%20Component%20Object%20Reference) (OtherBodyIndex :type Integer))
  (Class|BIInteraction|ResetInteractionTrace(Message) OtherActor))

(event EventBeginPlay
  (bind _returnvalue (Actor|GetParentActor))
  (bind _returnvalue_2 (Actor|GetComponentsbyTag _returnvalue "/Script/Engine.ShapeComponent" "box"))
  (bind _output (Utilities|Array|Get(acopy) _returnvalue_2))
  (Utilities|FlowControl|Sequence
    (:then_0
      (Utilities|IsValid _output
        (:Is%20Valid
          (Variables|Default|SetBoxRef _output)
          (Collision|AssignOnComponentBeginOverlap (Variables|Default|GetBoxRef) (delegate Custom|OnComponentBeginOverlap_Event))
          (Collision|AssignOnComponentEndOverlap (Variables|Default|GetBoxRef) (delegate Custom|OnComponentEndOverlap_Event)))))
    (:then_1
      (Variables|Default|SetInteractWidgetCompRef (Utilities|Array|Get(acopy) (Actor|GetComponentsbyTag (Actor|GetParentActor) "/Script/UMG.WidgetComponent" "interact"))))))

(fn ConstructionScript)

(fn CanFocus
  (params (Character :type Actor%20Object%20Reference))
  (if (Variables|Default|GetCharNeedsToBeInBox)
    (return (Collision|IsOverlappingActor (Variables|Default|GetBoxRef) Character :!class /Script/Engine.PrimitiveComponent))
    (else
      (return true))))