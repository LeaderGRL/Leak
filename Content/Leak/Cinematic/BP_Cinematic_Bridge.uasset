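; Bridge cinematic trigger that plays a one-time, widget-based cutscene when its box is overlapped while IsDone is true.
; It adds the cinematic widget, teleports the first-person character's capsule to a child actor's location, then after a delay shows a skip prompt and enables input.
; Releasing Space removes both widgets, disables the trigger's input and switches the player's Scar to the pistol.
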(event OnComponentBeginOverlap(Box)
  (params (OverlappedComponent :type Primitive%20Component%20Object%20Reference) (OtherActor :type Actor%20Object%20Reference) (OtherComp :type Primitive%20Component%20Object%20Reference) (OtherBodyIndex :type Integer) (bFromSweep :type Boolean) (SweepResult :type Hit%20Result%20Structure%20%28by%20ref%29))
  (if (Variables|Default|GetIsDone)
    (bind _returnvalue (UserInterface|CreateWidget "/Game/Leak/Cinematic/WB_Cinematic_Bridge_V1.WB_Cinematic_Bridge_V1_C"))
    (UserInterface|Viewport|AddtoViewport _returnvalue 0)
    (bind _asbp_first_person_character (Utilities|Casting|CastToBP_FirstPersonCharacter OtherActor))
    (Transformation|SetRelativeLocation (Variables|/Script/Engine.Character|GetCapsuleComponent _asbp_first_person_character) (Transformation|GetSocketLocation (Variables|Default|GetChildActor) "None") false true)
    (Utilities|FlowControl|Delay 1.0)
    (bind _returnvalue_2 (UserInterface|CreateWidget "/Game/Leak/Cinematic/WB_TextSkip.WB_TextSkip_C"))
    (UserInterface|Viewport|AddtoViewport _returnvalue_2 0)
    (Input|EnableInput (Game|GetPlayerController 0))
    (Variables|Default|SetIsDone false)))

(event Input|KeyboardEvents|SpaceBar
  (params (Key :type Key%20Structure :default "None"))
  (:Released
    (bind _foundwidgets (Widget|GetAllWidgetsOfClass "/Game/Leak/Cinematic/WB_TextSkip.WB_TextSkip_C" false))
    (Widget|RemovefromParent _foundwidgets)
    (bind _foundwidgets_2 (Widget|GetAllWidgetsOfClass "/Game/Leak/Cinematic/WB_Cinematic_Bridge_V1.WB_Cinematic_Bridge_V1_C" false))
    (Widget|RemovefromParent _foundwidgets_2)
    (Input|DisableInput (Game|GetPlayerController 0))
    (Default|SwitchScartoPistol (stale OnComponentBeginOverlap(Box) _asbp_first_person_character))))

(fn ConstructionScript)