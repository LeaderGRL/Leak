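; A pickup pistol actor that the first-person character can attach to the hand socket or throw away with the pick input.
; A box overlap caches the character and opens a gate that allows pickup; pressing again while attached detaches the gun and starts the throw.
; A timeline scaled by TimeToFly sweeps it from the hand along the camera direction, then physics takes over on finish or hit.
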(event OnComponentBeginOverlap(Box)
  (params (OverlappedComponent :type Primitive%20Component%20Object%20Reference) (OtherActor :type Actor%20Object%20Reference) (OtherComp :type Primitive%20Component%20Object%20Reference) (OtherBodyIndex :type Integer) (bFromSweep :type Boolean) (SweepResult :type Hit%20Result%20Structure%20%28by%20ref%29))
  (bind _asbp_first_person_character (Utilities|Casting|CastToBP_FirstPersonCharacter OtherActor))
  (Variables|Default|SetChar%20Ref _asbp_first_person_character)
  (Utilities|FlowControl|Gate true) ; enters at Open
)

(event OnComponentEndOverlap(Box)
  (params (OverlappedComponent :type Primitive%20Component%20Object%20Reference) (OtherActor :type Actor%20Object%20Reference) (OtherComp :type Primitive%20Component%20Object%20Reference) (OtherBodyIndex :type Integer))
  (bind _char_ref (Variables|Default|GetChar%20Ref))
  (Utilities|FlowControl|Gate true) ; enters at Close
)

(event Input|EnhancedActionEvents|EnhancedInputActionIA_Pick
  (params (ActionValue :type Boolean) (ElapsedSeconds :type Float%20%28double-precision%29) (TriggeredSeconds :type Float%20%28double-precision%29) (InputAction :type Input%20Action%20Object%20Reference :default "/Game/FirstPerson/Input/Actions/IA_Pick.IA_Pick"))
  (bind _char_ref (Variables|Default|GetChar%20Ref))
  (bind _staticmesh (Variables|Default|GetStaticMesh))
  (bind _char_ref_2 (Variables|Default|GetChar%20Ref))
  (if (Utilities|IsValid (Variables|Default|GetChar%20Ref))
    (if (Variables|/Game/FirstPerson/Blueprints/BP_FirstPersonCharacter.BP_FirstPersonCharacter_C|GetPistol%20Attached (Variables|Default|GetChar%20Ref))
      (Transformation|DetachFromActor "KeepWorld" "KeepWorld" "KeepWorld")
      (Variables|/Game/FirstPerson/Blueprints/BP_FirstPersonCharacter.BP_FirstPersonCharacter_C|SetPistol%20Attached _char_ref_2 false)
      (Variables|/Game/FirstPerson/Blueprints/BP_FirstPersonCharacter.BP_FirstPersonCharacter_C|SetbHasRifle _char_ref_2 false)
      (Collision|SetCollisionEnabled _staticmesh "QueryAndPhysics")
      (|Throw)
      (else
        (Utilities|FlowControl|Gate true
          (:Exit
            (if (not (Variables|/Game/FirstPerson/Blueprints/BP_FirstPersonCharacter.BP_FirstPersonCharacter_C|GetPistol%20Attached (Variables|Default|GetChar%20Ref)))
              (Variables|/Game/FirstPerson/Blueprints/BP_FirstPersonCharacter.BP_FirstPersonCharacter_C|SetPistol%20Attached _char_ref true)
              (Variables|/Game/FirstPerson/Blueprints/BP_FirstPersonCharacter.BP_FirstPersonCharacter_C|SetbHasRifle _char_ref true)
              (bind _returnvalue (Transformation|AttachComponentToComponent (Variables|/Game/FirstPerson/Blueprints/BP_FirstPersonCharacter.BP_FirstPersonCharacter_C|GetFirstPersonMesh (Variables|Default|GetChar%20Ref)) "hand_rSocket" "SnapToTarget" "SnapToTarget" "SnapToTarget" true))
              (if _returnvalue
                (Physics|SetSimulatePhysics _staticmesh false)))))))))

(event Collision|EventHit
  (params (MyComp :type Primitive%20Component%20Object%20Reference) (Other :type Actor%20Object%20Reference) (OtherComp :type Primitive%20Component%20Object%20Reference) (bSelfMoved :type Boolean) (HitLocation :type Vector :default "0, 0, 0") (HitNormal :type Vector :default "0, 0, 0") (NormalImpulse :type Vector :default "0, 0, 0") (Hit :type Hit%20Result%20Structure%20%28by%20ref%29))
  (Audio|Components|Audio|Stop (Variables|Default|GetThrowingTL))
  (Physics|SetSimulatePhysics (Variables|Default|GetStaticMesh) true))

(fn ConstructionScript
  (Components|Timeline|SetPlayRate (Variables|Default|GetThrowingTL) (/ 1.0 (Variables|Default|GetTime%20to%20fly))))