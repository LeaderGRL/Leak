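; BP_Gun is an interactable gun the player can pick up and throw.
; A child custom-shape interaction area receives its mesh and interact duration at construction, and interface events toggle custom depth on focus.
; Interacting attaches it to the first-person character's hand socket and sets the throwable and rifle flags, unless a throwable is already held.
; Throw input detaches it, clears those flags and applies a camera-relative physics impulse.
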(event Custom|Interact
  (bind _char_ref (Variables|Components|GetChar%20Ref))
  (Variables|Default|SetInteractToggle (not (Variables|Default|GetInteractToggle)))
  (if (not (Variables|/Game/FirstPerson/Blueprints/BP_FirstPersonCharacter.BP_FirstPersonCharacter_C|GetHasThrowable (Variables|Components|GetChar%20Ref)))
    (Variables|/Game/FirstPerson/Blueprints/BP_FirstPersonCharacter.BP_FirstPersonCharacter_C|SetHasThrowable _char_ref true)
    (Variables|/Game/FirstPerson/Blueprints/BP_FirstPersonCharacter.BP_FirstPersonCharacter_C|SetbHasRifle _char_ref true)
    (Variables|Default|SetIsAttached true)
    (bind _returnvalue (Transformation|AttachComponentToComponent (Variables|/Game/FirstPerson/Blueprints/BP_FirstPersonCharacter.BP_FirstPersonCharacter_C|GetFirstPersonMesh (Variables|Components|GetChar%20Ref)) "hand_rSocket" "SnapToTarget" "SnapToTarget" "SnapToTarget" true))
    (if _returnvalue
      (Physics|SetSimulatePhysics (Variables|Default|GetStaticMesh) false))))

(event Input|EnhancedActionEvents|EnhancedInputActionIA_Throw
  (params (ActionValue :type Boolean) (ElapsedSeconds :type Float%20%28double-precision%29) (TriggeredSeconds :type Float%20%28double-precision%29) (InputAction :type Input%20Action%20Object%20Reference :default "/Game/FirstPerson/Input/Actions/IA_Throw.IA_Throw"))
  (bind _staticmesh (Variables|Default|GetStaticMesh))
  (bind _char_ref (Variables|Components|GetChar%20Ref))
  (if (Variables|Default|GetIsAttached)
    (Transformation|DetachFromActor "KeepWorld" "KeepWorld" "KeepWorld")
    (Variables|/Game/FirstPerson/Blueprints/BP_FirstPersonCharacter.BP_FirstPersonCharacter_C|SetHasThrowable _char_ref false)
    (Variables|/Game/FirstPerson/Blueprints/BP_FirstPersonCharacter.BP_FirstPersonCharacter_C|SetbHasRifle _char_ref false)
    (Variables|Default|SetIsAttached false)
    (Collision|SetCollisionEnabled _staticmesh "QueryAndPhysics")
    (Physics|SetSimulatePhysics _staticmesh true)
    (Physics|AddImpulse (Variables|Default|GetStaticMesh) (* (Math|Vector|RotateVector (Math|Vector|MakeVector 1e+03 0.0 (Variables|Default|GetThrowHeight)) (Camera|GetCameraRotation (Game|GetPlayerCameraManager 0))) (Variables|Default|GetPowzree)) "None" false)))

(event EventInterfaceInteract
  (CallFunction|Interact))

(event EventInterfaceToggleFocus
  (params (Focus :type Boolean))
  (Rendering|SetRenderCustomDepth (Variables|Default|GetStaticMesh) Focus))

(event EventBeginPlay
  (bind _asbp_first_person_character (Utilities|Casting|CastToBP_FirstPersonCharacter (Game|GetPlayerCharacter 0)))
  (Variables|Components|SetChar%20Ref _asbp_first_person_character))

(fn ConstructionScript
  (bind _asbp_interaction_area_custom_shape (Utilities|Casting|CastToBP_InteractionArea_Custom_Shape (Variables|/Script/Engine.ChildActorComponent|GetChildActor (Variables|Default|GetChildActor))))
  (Variables|/Game/Interaction/InteractionArea/BP_InteractionArea_Master.BP_InteractionArea_Master_C|SetInteractDuration _asbp_interaction_area_custom_shape (Variables|Default|GetInteract%20Duration))
  (Variables|/Game/Interaction/InteractionArea/BP_InteractionArea_Custom_Shape.BP_InteractionArea_Custom_Shape_C|SetShape _asbp_interaction_area_custom_shape (Variables|Default|GetStaticMesh)))

(fn GetInteractionWidgetRef
  (return (Variables|Default|GetWidget)))