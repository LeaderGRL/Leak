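; BP_Puzzle_test is a test interactable puzzle that moves the player's view to its own camera and hands input to an on-object widget.
; The construction script sets the camera transform and FOV, and BeginPlay retries until WidgetTest exists to set itself as parent.
; Focus toggles custom depth; interacting blends to the camera with cursor and UI-only input.
; EndPuzzle returns the view to the character without restoring input.
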(event Custom|InteractOnServer
  (bind _returnvalue (Game|GetPlayerController 0))
  (Variables|Default|SetInteractToggle (not (Variables|Default|GetInteractToggle)))
  (CallFunction|MoveCamera _returnvalue self)
  (Variables|/Script/Engine.PlayerController|SetbShowMouseCursor _returnvalue true)
  (Input|SetInputModeUIOnly _returnvalue (UserInterface|GetWidget (Variables|Default|GetWidget1)) "DoNotLock" true))

(event EventBeginPlay
  (bind _aswidget_test (Utilities|Casting|CastToWidgetTest (UserInterface|GetWidget (Variables|Default|GetWidget1)) :!label _label)
    (:then
      (Variables|/Game/Test/WidgetTest.WidgetTest_C|Setparent _aswidget_test self))
    (:CastFailed
      (Utilities|FlowControl|Delay 0.1)
      (goto _label))))

(event EventEndPuzzle
  (Game|Player|SetViewTargetwithBlend (Game|GetPlayerController 0) (Game|GetPlayerCharacter 0) 0.0 "VTBlend_Linear" 0.0 false))

(event EventInterfaceToggleFocus
  (params (Focus :type Boolean))
  (Rendering|SetRenderCustomDepth (Variables|Default|GetPuzzleObject) Focus))

(event EventInterfaceInteract
  (CallFunction|InteractonServer))

(fn ConstructionScript
  (bind _camera_rotation (Variables|Default|GetCamera%20Rotation))
  (bind _camera (Variables|Default|GetCamera))
  (bind (_roll _pitch _yaw) (Math|Rotator|BreakRotator _camera_rotation))
  ;[0 1 0.9062] Set Camera Parameters
  (Transformation|SetRelativeLocationAndRotation _camera (Variables|Default|GetCamera%20Location) _camera_rotation false false)
  (Variables|Default|SetPitch _pitch)
  (Variables|Default|SetYaw _yaw)
  (Camera|SetFieldOfView _camera (Variables|Default|GetCamera%20FOV)))

(fn MoveCamera
  (params (From :type Player%20Controller%20Object%20Reference) (To :type Actor%20Object%20Reference))
  (Game|Player|SetViewTargetwithBlend From To 1.0 "VTBlend_Linear" 0.0 false))