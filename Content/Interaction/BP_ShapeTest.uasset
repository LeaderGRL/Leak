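; BP_ShapeTest is a test interactable actor that implements focus and interact interface events.
; Focus toggles custom depth rendering on its Cone mesh, and a getter exposes its interaction Widget.
; Interacting calls InteractOnServer, which flips the InteractToggle variable, whose RepNotify prints a debug string to check replication.
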(event Custom|InteractOnServer
  (Variables|Default|SetInteractToggle (not (Variables|Default|GetInteractToggle))))

(event EventInterfaceToggleFocus
  (params (Focus :type Boolean))
  (Rendering|SetRenderCustomDepth (Variables|Default|GetCone) Focus))

(event EventInterfaceInteract
  (CallFunction|InteractonServer))

(fn ConstructionScript)

(fn OnRepInteractToggle
  (Development|PrintString "testHello"))

(fn GetInteractionWidgetRef
  (return (Variables|Default|GetWidget)))